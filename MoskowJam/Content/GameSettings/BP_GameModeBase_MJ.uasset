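; Game mode for a cat-crewed submarine level, handling crisis reactions and end-game conditions.
; On BeginPlay it caches the NPC manager, cats and lamps, then binds to submarine and trap spawner events.
; Submarine events recolor lamps; damage also shakes the camera and temporarily panics cats, adding stress.
; Enough traps, zero HP or too many angry cats trigger the end-game screen; RegenStamina restores free cats' stamina and stress.
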(event `self.ReceiveBeginPlay`
  (`|ExecutionSequence`
    (:`then_0`
      (bind _outactors (`GameplayStatics.GetAllActorsOfClass` "/Game/Actors/Environment/BP_NPC_Manager.BP_NPC_Manager_C"))
      ;[0.6667 0 0.05239] Все делаеться в каждой итерации цикла( да она одна, но это ничем не гарантировано)
      (for _array_element _outactors
        (bind _output_get (set `self.NPC Manager` _array_element))
        (bind _array_of_cats (`/Game/Actors/Environment/BP_NPC_Manager.Get Array of Cats` _output_get))
        (set `self.Array Of Cats` _array_of_cats)
        (bind _outactors_2 (`GameplayStatics.GetAllActorsOfClass` "/Game/ART/BP_Lamp.BP_Lamp_C"))
        (set `self.Array of Lamps` _outactors_2)
        (bind _outactors_3 (`GameplayStatics.GetAllActorsOfClass` "/Game/Test/BP_Submarine.BP_Submarine_C"))
        (for _array_element_2 _outactors_3
          (bind _output_get_2 (set `self.Submarine` _array_element_2))
          (add `Submarine.OnChangedCurrentHPEvent` _output_get_2 (delegate `Submarine Taken Damage`))
          (add `/Game/Test/BP_Submarine.Barier Located` (`self.Submarine`) (delegate `Barier Located Helper`))
          (add `/Game/Test/BP_Submarine.End of Location` (`self.Submarine`) (delegate `End of Location Helper`)))))
    (:`then_1`
      (bind _outactors_4 (`GameplayStatics.GetAllActorsOfClass` "/Script/MoskowJam.Spawner"))
      (for _array_element_3 _outactors_4
        (add `Spawner.OnSpawnTrapEvent` _array_element_3 (delegate `SpawnTrap`))))))

(event `Barier Located Helper`
  (params (TrupDetected :type "/Game/Actors/Environment/Barrier/Traps/BP_Traps Object Reference"))
  (for _array_element (`self.Array of Lamps`)
    (`/Game/ART/BP_Lamp.Change color to Orange` _array_element)))

(event `End of Location Helper`
  (for _array_element (`self.Array of Lamps`)
    (`/Game/ART/BP_Lamp.Change color to Normal` _array_element)))

(event `SpawnTrap`
  (params (CounterTrap :type Integer) (Traps :type "Barrier Object Reference"))
  ;[1 1 1] Условия победы
  (if (>= CounterTrap (`self.TrapForWin`))
    (`/Game/Library/FL_General.Create End Game Statistic` "None")))

(event `Submarine Taken Damage`
  (params (NewVal :type "Float (single-precision)"))
  (bind _output_get (set `self.Submarine HP` NewVal))
  (if (> _output_get 0.0)
    ;[1 1 1] Реагирование на дамаг подлодки: тряска камеры игрока, смены цвета ламп, паника котов, задержка 5 сек, нормальный свет, задержка 1 сек, снятие паники у котов
    (bind _asbp_player_character (cast `/Game/Actors/Player_Character/BP_Player_Character` (`GameplayStatics.GetPlayerCharacter` 0)))
    (`/Game/Actors/Player_Character/BP_Player_Character.Shaking Camera` _asbp_player_character)
    (for _array_element (`self.Array of Lamps`)
      (`/Game/ART/BP_Lamp.Change color to Red` _array_element))
    (for _array_element_2 (`self.Array Of Cats`)
      (message `/Game/Interfaces/IBP_Tags_Management.Add Tag` _array_element_2 (struct :`TagName` "Anim.Panic"))
      (message `/Game/Interfaces/IBP_HR.Increase Stress` _array_element_2 10.0))
    (`KismetSystemLibrary.Delay` 5.0)
    (for _array_element_3 (`self.Array of Lamps`)
      (`/Game/ART/BP_Lamp.Change color to Normal` _array_element_3))
    (`KismetSystemLibrary.Delay` 1.0)
    (for _array_element_4 (`self.Array Of Cats`)
      (message `/Game/Interfaces/IBP_Tags_Management.Remove Tag` _array_element_4 (struct :`TagName` "Anim.Panic")))
    (else
      (`/Game/Library/FL_General.Create End Game Statistic` (`self.Level Name To Button Left`) (`self.Level Name To Button Right`) (`self.Left Button Text`) (`self.Right Button Text`) (`self.Result`) (`self.Text Message`)))))

(event `Regen Stamina`
  ;[1 1 1] К этому событию подключён таймер в NPC Manager, это событие отвечает за реген стамины и стресса
  (bind _array_of_free_cats (`/Game/Actors/Environment/BP_NPC_Manager.Get Array of Free Cats` (`self.NPC Manager`)))
  (for _array_element _array_of_free_cats
    (message `/Game/Interfaces/IBP_HR.Regen Stamina` _array_element 5.0)
    (message `/Game/Interfaces/IBP_HR.Regen Stress` _array_element 1.0)))

(fn `Increase Angry Cats Counter`
  (bind _result (`/Engine/EditorBlueprintResources/StandardMacros.IncrementInt` (`self.Angry Cats Counter`))
    (:`  `
      (if (> _result (`self.Max Angry Cats`))
        (`/Game/Library/FL_General.Create End Game Statistic` "MaimMenu_Level" "Test_Level_Karbiorn" "Вернуться в меню" "Попробовать еще раз" "Поражение" "К сожалению, уровень стресса котиков на подлодке слишком высокий, поэтому придётся вернуться, немного отдохнуть и попробовать снова.")))))

(fn `UserConstructionScript`)