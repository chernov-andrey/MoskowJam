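; Player controller for a submarine game that owns Enhanced Input contexts, relays interact input and opens the pause menu.
; It adds the default context on BeginPlay, offers functions to add, remove or swap contexts, and broadcasts E/F presses through dispatchers.
; Widget references guard against duplicates and clear through close callbacks.
; Many debug keys test submarine movement, HP, torpedoes, shark spawning, lamps, sailor cat messages and message or end-game screens.
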(event Custom|Closed%20Helper
  ;[1 1 1] Дебаг
  ;;[1 1 1] Вывод текстового сообщения. ДО и после вывода сообщения делать паузу и задержку, иначе инпут сломается
  (Variables|Default|SetText%20Widget 0)
  (Utilities|FlowControl|Delay 0.5)
  (Game|SetGamePaused false))

(event Custom|Pause%20Closed%20Helper
  ;[1 1 1] Пауза
  (Variables|Default|SetPause%20Widget 0))

(event Custom|End%20Closed%20Event
  ;[1 1 1] Дебаг
  ;;[1 1 1] Вызов экрана статистики
  (Variables|Default|SetEnd%20WIdget 0)
  (Utilities|FlowControl|Delay 0.5)
  (Game|SetGamePaused false))

(event Input|EnhancedActionEvents|EnhancedInputActionIA_Interact_1
  (params (ActionValue :type Boolean) (ElapsedSeconds :type Float%20%28double-precision%29) (TriggeredSeconds :type Float%20%28double-precision%29) (InputAction :type Input%20Action%20Object%20Reference :default "/Game/GameSettings/InputActions/IA_Interact_1.IA_Interact_1"))
  ;[1 1 1] Вызов взаимодействия
  (Default|CallEPressed))

(event Input|EnhancedActionEvents|EnhancedInputActionIA_Interact_2
  (params (ActionValue :type Boolean) (ElapsedSeconds :type Float%20%28double-precision%29) (TriggeredSeconds :type Float%20%28double-precision%29) (InputAction :type Input%20Action%20Object%20Reference :default "/Game/GameSettings/InputActions/IA_Interact_2.IA_Interact_2"))
  ;[1 1 1] Обрабатываем нажатие кнопки F
  (Default|CallFPressed))

(event Input|EnhancedActionEvents|EnhancedInputActionIA_Pause
  (params (ActionValue :type Boolean) (ElapsedSeconds :type Float%20%28double-precision%29) (TriggeredSeconds :type Float%20%28double-precision%29) (InputAction :type Input%20Action%20Object%20Reference :default "/Game/GameSettings/InputActions/IA_Pause.IA_Pause"))
  ;[1 1 1] Пауза
  (Game|SetGamePaused true)
  (Utilities|IsValid (Variables|Default|GetPause%20Widget)
    (:Is%20Not%20Valid
      (bind _returnvalue (CallFunction|CreatePauseWidget))
      (bind _output_get (Variables|Default|SetPause%20Widget _returnvalue))
      (EventDispatchers|BindEventtoPauseClosed _output_get (delegate Custom|Pause%20Closed%20Helper)))))

(event EventBeginPlay
  (bind _returnvalue (PlayerController|LocalPlayerSubsystems|GetEnhancedInputLocalPlayerSubsystem))
  ;[1 1 1] Подключение контекста управления
  (Utilities|IsValid _returnvalue
    (:Is%20Valid
      (Input|AddMappingContext _returnvalue "/Game/GameSettings/IMC_Default.IMC_Default" 0 "(bIgnoreAllPressedKeysUntilRelease=True,bForceImmediately=False,bNotifyUserSettings=False)"))))

(event Input|KeyboardEvents|DebugKeyT
  (params (Key :type Key%20Structure :default "None") (ActionValue :type Input%20Action%20Value%20Structure))
  ;[1 1 1] Дебаг
  ;;[1 1 1] Вывод текстового сообщения. ДО и после вывода сообщения делать паузу и задержку, иначе инпут сломается
  (:Pressed
    (Utilities|IsValid (Variables|Default|GetText%20Widget)
      (:Is%20Not%20Valid
        (bind _text_widget (CallFunction|CreateMessageWidget "Тест текстового сообщения. Тут можно будет вывести обучение, например. Сейчас это сообщение обучает тому, что может это сообщение. Работает, получается."))
        (bind _output_get (Variables|Default|SetText%20Widget _text_widget))
        (EventDispatchers|BindEventtoClosed _output_get (delegate Custom|Closed%20Helper))))))

(event Input|KeyboardEvents|DebugKeyY
  (params (Key :type Key%20Structure :default "None") (ActionValue :type Input%20Action%20Value%20Structure))
  ;[1 1 1] Дебаг
  ;;[1 1 1] Вызов экрана статистики
  (:Pressed
    (Game|SetGamePaused true)
    (Utilities|FlowControl|Delay 0.5)
    (Utilities|IsValid (Variables|Default|GetEnd%20WIdget)
      (:Is%20Not%20Valid
        (bind _end_widget (CallFunction|CreateEndGameStatistic "Test_Build" "Test_Level_Karbiorn" "Тест Корабль" "Тест Уровень" "Вы нажали Y" "Это отладка текстового сообщения финала"))
        (bind _output_get (Variables|Default|SetEnd%20WIdget _end_widget))
        (EventDispatchers|BindEventtoClosed _output_get (delegate Custom|End%20Closed%20Event))))))

(event Input|KeyboardEvents|DebugKeyG
  (params (Key :type Key%20Structure :default "None") (ActionValue :type Input%20Action%20Value%20Structure))
  ;[1 1 1] Дебаг
  ;;[1 1 1] Спаун торпеды
  (:Pressed
    (bind _returnvalue (CallFunction|GetSubmarine))
    (bind _asbp_submarine (Utilities|Casting|CastToBP_Submarine _returnvalue))
    (Default|SpawnMissle _asbp_submarine)))

(event Input|KeyboardEvents|DebugKeyB
  (params (Key :type Key%20Structure :default "None") (ActionValue :type Input%20Action%20Value%20Structure))
  ;[1 1 1] Дебаг
  ;;[1 1 1] В случае получения подлодкой урона - запустить эту последовательность
  (:Pressed
    (bind _returnvalue (CallFunction|GetSubmarine))
    (Class|Submarine|ChangeHP _returnvalue 1e+01)))

(event Input|KeyboardEvents|DebugKeyC
  (params (Key :type Key%20Structure :default "None") (ActionValue :type Input%20Action%20Value%20Structure))
  ;[1 1 1] Дебаг
  (:Pressed
    (bind _outactors (Actor|GetAllActorsOfClass "/Game/Actors/Bots/BP_Cat_Sailor.BP_Cat_Sailor_C"))
    (for _array_element _outactors
      (bind _output_get (Variables|Default|SetArray%20Element _array_element)))
    (Class|IBPHR|WorkResultMessage(Message) _output_get "Вы супер!")))

(event Input|KeyboardEvents|DebugKeyI
  (params (Key :type Key%20Structure :default "None") (ActionValue :type Input%20Action%20Value%20Structure))
  ;[1 1 1] Дебаг
  ;;[1 1 1] Дебаг скорости и поворотов подлодки
  (:Pressed
    (Class|Submarine|ChangeCurrentSpeed (Class|MBFLSubmarine|GetSubmarine self) 5e+02)))

(event Input|KeyboardEvents|DebugKeyJ
  (params (Key :type Key%20Structure :default "None") (ActionValue :type Input%20Action%20Value%20Structure))
  ;[1 1 1] Дебаг
  ;;[1 1 1] Дебаг скорости и поворотов подлодки
  (:Pressed
    (Class|Submarine|ChangeCurrentSpeed (Class|MBFLSubmarine|GetSubmarine self) -5e+02)))

(event Input|KeyboardEvents|DebugKeyJ
  (params (Key :type Key%20Structure :default "None") (ActionValue :type Input%20Action%20Value%20Structure))
  ;[1 1 1] Дебаг
  ;;[1 1 1] Дебаг скорости и поворотов подлодки
  (:Pressed
    (Class|Submarine|ChangeCurrentRotation (Class|MBFLSubmarine|GetSubmarine self) "0.000000,-10.000000,0.000000")))

(event Input|KeyboardEvents|DebugKeyL
  (params (Key :type Key%20Structure :default "None") (ActionValue :type Input%20Action%20Value%20Structure))
  ;[1 1 1] Дебаг
  ;;[1 1 1] Дебаг скорости и поворотов подлодки
  (:Pressed
    (Class|Submarine|ChangeCurrentRotation (Class|MBFLSubmarine|GetSubmarine self) "0.000000,10.000000,0.000000")))

(event Input|KeyboardEvents|DebugKeyN
  (params (Key :type Key%20Structure :default "None") (ActionValue :type Input%20Action%20Value%20Structure))
  ;[1 1 1] Дебаг
  (:Pressed
    (bind _returnvalue (CallFunction|GetSubmarine))
    (bind _asbp_submarine (Utilities|Casting|CastToBP_Submarine _returnvalue))
    (bind _barier_detector_location (Default|GetBarierLocation _asbp_submarine))
    (bind _returnvalue_2 (Game|SpawnActorfromClass "/Game/Actors/Environment/Barrier/Traps/Traps_Iteractive/Creatures/BP_Creature_Shark.BP_Creature_Shark_C" (Math|Transform|MakeTransform _barier_detector_location "0, 0, 0" "1.000000,1.000000,1.000000") "Undefined" "MultiplyWithRoot" _asbp_submarine 0))
    (Utilities|FlowControl|Delay 15.0)
    (Actor|DestroyActor _returnvalue_2)))

(event Input|KeyboardEvents|DebugKeyM
  (params (Key :type Key%20Structure :default "None") (ActionValue :type Input%20Action%20Value%20Structure))
  ;[1 1 1] Дебаг
  ;;[1 1 1] Когда всё вернулось в норм - запустить эту последовательность
  (:Pressed
    (bind _outactors (Actor|GetAllActorsOfClass "/Game/ART/BP_Lamp.BP_Lamp_C"))
    (for _array_element _outactors
      (Default|ChangeColortoNormal _array_element))))

(fn ConstructionScript)

(fn ChangeMappingContext
  (params (MappingContext :type Input%20Mapping%20Context%20Object%20Reference))
  (bind _returnvalue (PlayerController|LocalPlayerSubsystems|GetEnhancedInputLocalPlayerSubsystem))
  (Utilities|IsValid _returnvalue
    (:Is%20Valid
      (Input|RemoveMappingContext _returnvalue "/Game/GameSettings/IMC_Commander_Panel.IMC_Commander_Panel" "(bIgnoreAllPressedKeysUntilRelease=True,bForceImmediately=False,bNotifyUserSettings=False)")
      (Input|RemoveMappingContext _returnvalue "/Game/GameSettings/IMC_Default.IMC_Default" "(bIgnoreAllPressedKeysUntilRelease=True,bForceImmediately=False,bNotifyUserSettings=False)")
      (Input|AddMappingContext _returnvalue MappingContext 1 "(bIgnoreAllPressedKeysUntilRelease=True,bForceImmediately=False,bNotifyUserSettings=False)"))))

(fn AddMappingContext
  (params (MappingContext :type Input%20Mapping%20Context%20Object%20Reference))
  (bind _returnvalue (PlayerController|LocalPlayerSubsystems|GetEnhancedInputLocalPlayerSubsystem))
  (Utilities|IsValid _returnvalue
    (:Is%20Valid
      (Input|AddMappingContext _returnvalue MappingContext 1 "(bIgnoreAllPressedKeysUntilRelease=True,bForceImmediately=False,bNotifyUserSettings=False)"))))

(fn RemoveMappingContext
  (params (MappingContext :type Input%20Mapping%20Context%20Object%20Reference))
  (bind _returnvalue (PlayerController|LocalPlayerSubsystems|GetEnhancedInputLocalPlayerSubsystem))
  (Utilities|IsValid _returnvalue
    (:Is%20Valid
      (Input|RemoveMappingContext _returnvalue MappingContext "(bIgnoreAllPressedKeysUntilRelease=True,bForceImmediately=False,bNotifyUserSettings=False)"))))