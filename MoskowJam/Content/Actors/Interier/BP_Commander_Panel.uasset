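; BP_Commander_Panel is an interior actor that opens the commander menu when a player-tagged actor enters its Box trigger.
; On overlap it stores that actor as Commander, then creates BPW_CommanderMenu and adds it to the viewport at a fixed position.
; It then switches BP_PlayerController_MJ to the commander panel input mapping context and shows the mouse cursor after a short delay.
; No logic here closes the menu or restores input.
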(event `self.Box.OnComponentBeginOverlap`
  (params (OverlappedComponent :type "PrimitiveComponent Object Reference") (OtherActor :type "Actor Object Reference") (OtherComp :type "PrimitiveComponent Object Reference") (OtherBodyIndex :type Integer) (bFromSweep :type Boolean) (SweepResult :type "HitResult Structure (by ref)"))
  (if (`self.ActorHasTag` OtherActor "Player")
    (set `self.Commander` OtherActor)
    ;[1 1 1] Создание виджета коммандирского окна, спрятать в функцию, а функцию - в библиотеку функций
    (bind _returnvalue (`|CreateWidget` "/Game/GUI/BPW_CommanderMenu.BPW_CommanderMenu_C"))
    (bind _output_get (set `self.Commander Panel` _returnvalue))
    (`UserWidget.SetPositionInViewport` _output_get (600.0 400.0) true)
    (`UserWidget.AddToViewport` _output_get 0)
    (bind _asbp_player_controller_mj (cast `/Game/GameSettings/BP_PlayerController_MJ` (`GameplayStatics.GetPlayerController` 0)))
    (`/Game/GameSettings/BP_PlayerController_MJ.Change Mapping Context` _asbp_player_controller_mj "/Game/GameSettings/IMC_Commander_Panel.IMC_Commander_Panel")
    (`KismetSystemLibrary.Delay` 1.0)
    (set `PlayerController.bShowMouseCursor` true _asbp_player_controller_mj)))

(fn `UserConstructionScript`)