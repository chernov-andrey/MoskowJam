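; BP_Decoration2 is an environment decoration that shows a randomly picked Paper2D sprite on the surface beneath its spawn point.
; On BeginPlay it chooses the sprite and a random ±90 yaw offset, then line-traces downward, moving to the hit location or destroying itself when nothing is hit.
; Every Tick it billboards the sprite toward the submarine's location, using the stored offset to randomly vary which side faces it.
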(event `self.ReceiveBeginPlay`
  (bind _returnvalue (`self.K2_GetActorLocation`))
  (set `self.Rotation` (`KismetMathLibrary.SelectFloat` -90.0 90.0 (`KismetMathLibrary.RandomBool`)))
  (`PaperSpriteComponent.SetSprite` (`self.PaperSprite`) (`KismetArrayLibrary.Array_Random` (`self.Sprites`)))
  (bind (_outhit _returnvalue_2) (`KismetSystemLibrary.LineTraceSingle` _returnvalue (+ _returnvalue (0.0 0.0 -20000.0)) "TraceTypeQuery1"))
  (if _returnvalue_2
    (`self.K2_SetActorLocation` (`.Location` (`GameplayStatics.BreakHitResult` _outhit)))
    (else
      (`self.K2_DestroyActor`))))

(event `self.ReceiveTick`
  (params (DeltaSeconds :type "Float (single-precision)"))
  (`SceneComponent.K2_SetWorldRotation` (`self.PaperSprite`) (`KismetMathLibrary.Conv_VectorToRotator` (`KismetMathLibrary.GreaterGreater_VectorRotator` (- (`MBFL_Submarine.GetLocationSubmarine` self) (`self.K2_GetActorLocation`)) (`KismetMathLibrary.MakeRotator` 0.0 0.0 (`self.Rotation`)))) false false))

(fn `UserConstructionScript`)