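; Interactive shark creature trap that faces the submarine on spawn and swims with added speed, correcting sideways toward it until within an adjustment distance.
; On first hit with the submarine it plays a timed attack loop, then turns and swims away faster.
; A missile hit instead plays the death animation and drifts it upward.
; Both outcomes zero its world speed multiplier, clear the submarine's accident status after a delay, then destroy the shark.
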(event `self.ReceiveBeginPlay`
  (`self.K2_SetActorRotation` self (`KismetMathLibrary.FindLookAtRotation` (`self.K2_GetActorLocation` self) (`self.K2_GetActorLocation` (`MBFL_Submarine.GetSubmarine` self))) false)
  (`self.SetAdditionalSpeed` 300.0))

(event `self.StaticMeshComponent.OnComponentHit`
  (params (HitComponent :type "PrimitiveComponent Object Reference") (OtherActor :type "Actor Object Reference") (OtherComp :type "PrimitiveComponent Object Reference") (NormalImpulse :type "Vector Structure") (Hit :type "HitResult Structure (by ref)"))
  (if (== OtherActor (`MBFL_Submarine.GetSubmarine` self))
    (if (not (`self.IsTriggered`))
      (set `self.IsTriggered` true)
      (`SkeletalMeshComponent.PlayAnimation` (`self.SkeletalMesh`) "/Game/ART/AnimCharact/Shark/Animation/shark1_attack.shark1_attack" true)
      (`KismetSystemLibrary.Delay` 15.0)
      (`SkeletalMeshComponent.PlayAnimation` (`self.SkeletalMesh`) "/Game/ART/AnimCharact/Shark/Animation/shark1_swim.shark1_swim" true)
      (`SceneComponent.K2_SetRelativeRotation` (`self.SkeletalMesh`) (struct :`Yaw` -45.0) false false)
      (set `self.AdditionalMoveDirection` (-1.0 -1.0 0.0))
      (`self.SetAdditionalSpeed` 1000.0)
      (set `self.WorldSpeedMultiplier` 0.0 :!label _label)
      (`KismetSystemLibrary.Delay` 5.0)
      (`Submarine.SetAccidentStatus` (`MBFL_Submarine.GetSubmarine` self) false)
      (`KismetSystemLibrary.Delay` 10.0)
      (`self.K2_DestroyActor`))))

(event `/Game/Actors/Environment/Barrier/Traps/Traps_Iteractive/BI_InteractWithEnvironment.MissileHit`
  (`SkeletalMeshComponent.PlayAnimation` (`self.SkeletalMesh`) "/Game/ART/AnimCharact/Shark/Animation/shark1_dead.shark1_dead" false)
  (set `self.AdditionalMoveDirection` (0.0 0.0 1.0))
  (`self.SetAdditionalSpeed` 300.0)
  (goto _label))

(event `/Game/Actors/Environment/Barrier/Traps/Traps_Iteractive/BI_InteractWithEnvironment.Beep`)

(event `self.ReceiveTick`
  (params (DeltaSeconds :type "Float (single-precision)"))
  (bind _returnvalue (`self.K2_GetActorLocation`))
  (bind _returnvalue_2 (`MBFL_Submarine.GetLocationSubmarine` self))
  (bind _returnvalue_3 (- (.y _returnvalue_2) (.y _returnvalue)))
  (if (> (`KismetMathLibrary.Vector_Distance` _returnvalue_2 _returnvalue) (`self.PositionAdjustmentDistance`))
    (set `self.AdditionalMoveDirectionCorrect` (`KismetMathLibrary.MakeVector` 0.0 (`KismetMathLibrary.SelectFloat` _returnvalue_3 0.0 (> (`KismetMathLibrary.Abs` _returnvalue_3) 50.0))))))

(fn `Read Case`
  (returns (`Cat Case` :type "/Game/GUI/BPW_Cat_Case Object Reference"))
  (return null))

(fn `UserConstructionScript`)