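; BP_D_Rif is a destructible environment barrier actor built on a Chaos Geometry Collection.
; Its DestroyRIF event shatters the collection with a very strong external strain at the actor's location, then scatters the pieces with a radial velocity impulse.
; The Chaos break event only prints a debug message.
; A delayed collision shutoff exists in the graph but is unconnected, so it never runs.
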(event `self.ReceiveBeginPlay`)

(event `self.GeometryCollection.OnChaosBreakEvent`
  (params (BreakEvent :type "ChaosBreakEvent Structure (by ref)"))
  (`KismetSystemLibrary.PrintString` "Разбився"))

(event `/Game/Interfaces/IBP_Test_Rif.Destroy RIF`
  (params (Target :type "Barrier Object Reference"))
  (`GeometryCollectionComponent.ApplyExternalStrain` (`self.GeometryCollection`) 0 (`self.K2_GetActorLocation` self) 6000.0 100 5.0 10000000.0)
  (`PrimitiveComponent.AddRadialImpulse` (`self.GeometryCollection`) (`self.K2_GetActorLocation` self) 500.0 1000.0 "RIF_Constant" true))

(fn `UserConstructionScript`)