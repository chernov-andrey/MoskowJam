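; Configurable submarine workstation actor whose job enum selects engine, wheel, torpedo handling, hole repair, water pump or horn.
; Construction and BeginPlay set the mesh per job; BeginPlay also finds the moving submarine.
; Player overlap shows a prompt and binds the controller's E event to a job switch.
; Simple jobs fire once; engine, wheel and pump swap input mapping contexts until E exits, with widgets for engine and pump.
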(event `self.ReceiveBeginPlay`
  (bind _outactors (`GameplayStatics.GetAllActorsOfClass` "/Game/Test/BP_Moving_Submarine.BP_Moving_Submarine_C"))
  (for _array_element _outactors
    (set `self.Array Element` _array_element))
  (set `self.Moving Submarine` (`self.Array Element`))
  ;[1 1 1] Проверяем, что все экземпляры этого класса "нашли" подлодку
  (`KismetSystemLibrary.PrintString` (`KismetStringLibrary.Concat_StrStr` (`|GetEnumeratorNameAsString` (`self.This Station Job`)) " ready;"))
  (switch `/Game/Enums/EWorkStations` (`self.This Station Job`)
    (:`NewEnumerator0`
      (set `self.This SMesh` "/Game/ART/Engine/engine.engine")
      (set `self.Static Mesh` false)
      (set `self.Simple Interaction` false :!label _label))
    (:`NewEnumerator1`
      (set `self.This SMesh` "/Game/ART/rull/Rull.Rull")
      (set `self.Static Mesh` false)
      (goto _label))
    (:`NewEnumerator2`
      (set `self.This Mesh` "/Game/ART/lewer2.lewer2")
      (set `self.Static Mesh` true)
      (set `self.Simple Interaction` true :!label _label_2))
    (:`NewEnumerator6`
      (set `self.This Mesh` "/Game/ART/torpeds/torpedsPolki.torpedsPolki")
      (set `self.Static Mesh` true)
      (goto _label_2))
    (:`NewEnumerator7`
      (set `self.This Mesh` "/Game/ART/torpeds/torpeds.torpeds")
      (set `self.Static Mesh` true)
      (goto _label_2))
    (:`NewEnumerator8`
      (goto _label_2))
    (:`NewEnumerator9`
      (goto _label))
    (:`NewEnumerator10`
      (goto _label_2)))
  (if (`self.Static Mesh`)
    (`StaticMeshComponent.SetStaticMesh` (`self.StaticMesh`) (`self.This Mesh`))
    (else
      (set `SkeletalMeshComponent.SkeletalMeshAsset` (`self.This SMesh`) (`self.SkeletalMesh`)))))

(event `self.ReceiveActorBeginOverlap`
  (params (OtherActor :type "Actor Object Reference"))
  ;[1 1 1] Если игрок подходит к месту активации, он может взаимодействовать, вызывая соответствующий эффект
  (bind _output_get (set `self.Player` OtherActor))
  (if (`self.ActorHasTag` _output_get "Player")
    (bind _asbp_player_controller_mj (cast `/Game/GameSettings/BP_PlayerController_MJ` (`self.GetInstigatorController` (`self.Player`))))
    (set `self.As BP Player Controller MJ` _asbp_player_controller_mj)
    (bind _shown (message `/Game/Interfaces/IBP_Player_Interaction.Interaction Widget Shown` (`self.Player`)))
    (if (not _shown)
      (message `/Game/Interfaces/IBP_Player_Interaction.Show Interaction Widget` (`self.Player`) self (`KismetTextLibrary.Conv_StringToText` (`|GetEnumeratorNameAsString` (`self.This Station Job`))) "E")
      (if (not (`self.Controlling`))
        (add `/Game/GameSettings/BP_PlayerController_MJ.E pressed` (`self.As BP Player Controller MJ`) (delegate `E Pressed Helper`)))
      (add `self.OnActorEndOverlap` (delegate `OnActorEndOverlap_Event`)))))

(event `OnActorEndOverlap_Event` :!signature `self.OnActorEndOverlap`
  (params (OverlappedActor :type "Actor Object Reference") (OtherActor :type "Actor Object Reference"))
  ;[1 1 1] Если игрок подходит к месту активации, он может взаимодействовать, вызывая соответствующий эффект
  (message `/Game/Interfaces/IBP_Player_Interaction.Collapse Interaction Widget` OtherActor self)
  (remove `/Game/GameSettings/BP_PlayerController_MJ.E pressed` (`self.As BP Player Controller MJ`) (delegate `E Pressed Helper`)))

(event `E Pressed Helper`
  ;[1 1 1] Если игрок подходит к месту активации, он может взаимодействовать, вызывая соответствующий эффект
  ;;[1 1 1] Подключаемся к устройству, получаем соответствующее управление
  (set `self.Controlling` true)
  (`KismetSystemLibrary.PrintString` "You pressed E, greate!")
  (message `/Game/Interfaces/IBP_Player_Interaction.Collapse Interaction Widget` (`self.Player`) self)
  (`self.Switch on Enter EWorkStations`)
  (`KismetSystemLibrary.PrintString` (`|GetEnumeratorNameAsString` (`self.This Station Job`)))
  (if (`self.Simple Interaction`)
    (set `self.Controlling` false)
    (else
      (add `/Game/GameSettings/BP_PlayerController_MJ.E pressed` (`self.As BP Player Controller MJ`) (delegate `Exit from interaction`))))
  (remove `/Game/GameSettings/BP_PlayerController_MJ.E pressed` (`self.As BP Player Controller MJ`) (delegate `E Pressed Helper`)))

(event `Exit from interaction`
  ;[1 1 1] Если игрок подходит к месту активации, он может взаимодействовать, вызывая соответствующий эффект
  ;;[1 1 1] Отключаемся от устройства, отключаем его управление
  (`self.Switch on Exit EWorkStations`)
  (remove `/Game/GameSettings/BP_PlayerController_MJ.E pressed` (`self.As BP Player Controller MJ`) (delegate `Exit from interaction`))
  (set `self.Controlling` false))

(fn `Engine`)

(fn `Get Torpedos`)

(fn `Launch Torpedos`)

(fn `Set Speed`
  (params (Speed :type "Float (double-precision)"))
  (locals (`Speed Scale` :type "Float (double-precision)" :default 10.0))
  (bind _output_get (set `self.Speed` (* Speed (`local.Speed Scale`))))
  (`/Game/Test/BP_Moving_Submarine.Engine` (`self.Moving Submarine`) _output_get))

(fn `Set Torpedos`)

(fn `Switch on Enter EWorkStations`
  (locals (`Local Player Controller` :type "/Game/GameSettings/BP_PlayerController_MJ Object Reference") (`As BPW Water Pump` :type "/Game/GUI/BPW_WaterPump Object Reference"))
  (`/Game/GameSettings/BP_PlayerController_MJ.Set Moving Submarine` (`self.As BP Player Controller MJ`) (`self.Moving Submarine`))
  (bind _output_get (`/Game/Library/FL_General.Get  MJ Player Controller`))
  (set `local.Local Player Controller` _output_get)
  (switch `/Game/Enums/EWorkStations` (`self.This Station Job`)
    (:`NewEnumerator0`
      (`self.Engine`)
      (bind _widget (`/Game/Library/FL_General.Create Widget, Add to Viewport, Show mouse` "/Game/GUI/BPW_Engine_Slider.BPW_Engine_Slider_C"))
      (bind _output_get_2 (set `self.This Widget` _widget))
      (bind _asbpw_engine_slider (cast `/Game/GUI/BPW_Engine_Slider` _output_get_2))
      (`/Game/GUI/BPW_Engine_Slider.Set Owner` _asbpw_engine_slider self)
      (`/Game/GameSettings/BP_PlayerController_MJ.Add Mapping Context` (`local.Local Player Controller`) "/Game/GameSettings/IMC_Interaction_Zone.IMC_Interaction_Zone")
      (`/Game/GameSettings/BP_PlayerController_MJ.Remove Mapping Context` (`local.Local Player Controller`) "/Game/GameSettings/IMC_Default.IMC_Default"))
    (:`NewEnumerator1`
      (`self.Wheel`)
      (message `/Game/Interfaces/IBP_Moving_Submarine.Turn` (`self.Moving Submarine`) true)
      (`/Game/GameSettings/BP_PlayerController_MJ.Add Mapping Context` (`local.Local Player Controller`) "/Game/GameSettings/IMC_Wheel_Control.IMC_Wheel_Control")
      (`/Game/GameSettings/BP_PlayerController_MJ.Remove Mapping Context` (`local.Local Player Controller`) "/Game/GameSettings/IMC_Default.IMC_Default"))
    (:`NewEnumerator2`
      (`self.Launch Torpedos`)
      (bind _zero_torpedos (message `/Game/Interfaces/IBP_Moving_Submarine.Zero Torpedos?` (`self.Moving Submarine`)))
      (if _zero_torpedos
        (`KismetSystemLibrary.PrintString` "Торпедный аппарат пуст")
        (else
          (message `/Game/Interfaces/IBP_Moving_Submarine.:aunch Torpedos` (`self.Moving Submarine`)))))
    (:`NewEnumerator6`
      (`self.Get Torpedos`)
      (bind _max_torpedos (message `/Game/Interfaces/IBP_Moving_Submarine.Max Torpedos?` (`self.Moving Submarine`)))
      (if _max_torpedos
        (`KismetSystemLibrary.PrintString` "Торпедный аппарат полон")
        (else
          (message `/Game/Interfaces/IBP_Player_Interaction.Change Mesh in Hands and its Visibility` (`self.Player`) "/Game/ART/torpedo.torpedo" true "NewEnumerator2"))))
    (:`NewEnumerator7`
      (`self.Set Torpedos`)
      (bind _max_torpedos_2 (message `/Game/Interfaces/IBP_Moving_Submarine.Max Torpedos?` (`self.Moving Submarine`)))
      (if _max_torpedos_2
        (`KismetSystemLibrary.PrintString` "Торпедный аппарат полон")
        (else
          (bind _success (message `/Game/Interfaces/IBP_Player_Interaction.Change Mesh in Hands and its Visibility` (`self.Player`) "/Game/ART/torpedo.torpedo" false "NewEnumerator2"))
          (if _success
            (message `/Game/Interfaces/IBP_Moving_Submarine.Load Torpedos` (`self.Moving Submarine`))
            (else
              (`KismetSystemLibrary.PrintString` "Ошибка помещения торпеды, руки пусты"))))))
    (:`NewEnumerator8`
      (`KismetSystemLibrary.PrintString` "Дыра заварена!")
      (message `/Game/Interfaces/IBP_Moving_Submarine.Hole Heal` (`self.Moving Submarine`) self))
    (:`NewEnumerator9`
      (`KismetSystemLibrary.PrintString` "Насос работает")
      (`/Game/GameSettings/BP_PlayerController_MJ.Add Mapping Context` (`local.Local Player Controller`) "/Game/GameSettings/IMC_Pump_Control.IMC_Pump_Control")
      (`/Game/GameSettings/BP_PlayerController_MJ.Remove Mapping Context` (`local.Local Player Controller`) "/Game/GameSettings/IMC_Default.IMC_Default")
      (bind _widget_2 (`/Game/Library/FL_General.Create Widget, Add to Viewport, Show mouse` "/Game/GUI/BPW_WaterPump.BPW_WaterPump_C"))
      (bind _output_get_3 (set `self.This Widget` _widget_2))
      (bind _asbpw_water_pump (cast `/Game/GUI/BPW_WaterPump` _output_get_3))
      (bind _output_get_4 (set `local.As BPW Water Pump` _asbpw_water_pump))
      (`/Game/GUI/BPW_WaterPump.Set Owner` _output_get_4 (`self.Moving Submarine`)))
    (:`NewEnumerator10`
      (`GameplayStatics.PlaySoundAtLocation` "/Game/Sound/Cue_Sound/Effects/Котосирена_Cue.Котосирена_Cue" (`self.K2_GetActorLocation` self) (struct) 1.0 1.0 0.0 null null null null))))

(fn `Switch on Exit EWorkStations`
  (switch `/Game/Enums/EWorkStations` (`self.This Station Job`)
    (:`NewEnumerator0`
      (bind _output_get (`/Game/Library/FL_General.Get  MJ Player Controller`))
      (`/Game/GameSettings/BP_PlayerController_MJ.Remove Mapping Context` _output_get "/Game/GameSettings/IMC_Interaction_Zone.IMC_Interaction_Zone")
      (`/Game/GameSettings/BP_PlayerController_MJ.Add Mapping Context` _output_get "/Game/GameSettings/IMC_Default.IMC_Default")
      (`Widget.RemoveFromParent` (`self.This Widget`))
      (`WidgetBlueprintLibrary.SetInputMode_GameOnly` _output_get)
      (set `PlayerController.bShowMouseCursor` false _output_get))
    (:`NewEnumerator1`
      (bind _output_get_2 (`/Game/Library/FL_General.Get  MJ Player Controller`))
      (`/Game/GameSettings/BP_PlayerController_MJ.Remove Mapping Context` _output_get_2 "/Game/GameSettings/IMC_Wheel_Control.IMC_Wheel_Control")
      (`/Game/GameSettings/BP_PlayerController_MJ.Add Mapping Context` _output_get_2 "/Game/GameSettings/IMC_Default.IMC_Default"))
    (:`NewEnumerator2`
      (`self.Launch Torpedos`))
    (:`NewEnumerator6`
      (`self.Get Torpedos`))
    (:`NewEnumerator7`
      (`self.Set Torpedos`))
    (:`NewEnumerator9`
      (bind _output_get_3 (`/Game/Library/FL_General.Get  MJ Player Controller`))
      (`/Game/GameSettings/BP_PlayerController_MJ.Remove Mapping Context` _output_get_3 "/Game/GameSettings/IMC_Pump_Control.IMC_Pump_Control")
      (`/Game/GameSettings/BP_PlayerController_MJ.Add Mapping Context` _output_get_3 "/Game/GameSettings/IMC_Default.IMC_Default")
      (`Widget.RemoveFromParent` (`self.This Widget`)))))

(fn `UserConstructionScript`
  (switch `/Game/Enums/EWorkStations` (`self.This Station Job`)
    (:`NewEnumerator0`
      (set `self.This SMesh` "/Game/ART/Engine/engine.engine")
      (set `self.Static Mesh` false))
    (:`NewEnumerator1`
      (set `self.This SMesh` "/Game/ART/rull/Rull.Rull")
      (set `self.Static Mesh` false))
    (:`NewEnumerator2`
      (set `self.This Mesh` "/Game/ART/lewer2.lewer2")
      (set `self.Static Mesh` true))
    (:`NewEnumerator6`
      (set `self.This Mesh` "/Game/ART/torpeds/torpedsPolki.torpedsPolki")
      (set `self.Static Mesh` true))
    (:`NewEnumerator7`
      (set `self.This Mesh` "/Game/ART/torpeds/torpeds.torpeds")
      (set `self.Static Mesh` true)))
  (if (`self.Static Mesh`)
    (`StaticMeshComponent.SetStaticMesh` (`self.StaticMesh`) (`self.This Mesh`))
    (else
      (set `SkeletalMeshComponent.SkeletalMeshAsset` (`self.This SMesh`) (`self.SkeletalMesh`)))))

(fn `Wheel`)