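; BP_Water is a water volume whose level rises with the number of holes and shows an underwater widget on the player.
; Tick grows the mesh's Z scale in proportion to NumsOfHoles, which ChangeNimsOfHoles increments or decrements.
; DecreaseWaterLevel lowers that scale in a single looped burst divided by WaterSpeed, clamped at zero.
; Actor overlap begin and end tell BP_Player_Character to create or remove the widget.
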(event `self.ReceiveBeginPlay`
  (add `self.OnActorBeginOverlap` (delegate `OnActorBeginOverlap_Event`))
  (add `self.OnActorEndOverlap` (delegate `OnActorEndOverlap_Event`)))

(event `OnActorBeginOverlap_Event` :!signature `self.OnActorBeginOverlap`
  (params (OverlappedActor :type "Actor Object Reference") (OtherActor :type "Actor Object Reference"))
  (bind _asbp_player_character (cast `/Game/Actors/Player_Character/BP_Player_Character` OtherActor))
  (`/Game/Actors/Player_Character/BP_Player_Character.Create Widget Under Water` _asbp_player_character))

(event `OnActorEndOverlap_Event` :!signature `self.OnActorEndOverlap`
  (params (OverlappedActor :type "Actor Object Reference") (OtherActor :type "Actor Object Reference"))
  (bind _asbp_player_character (cast `/Game/Actors/Player_Character/BP_Player_Character` OtherActor))
  (`/Game/Actors/Player_Character/BP_Player_Character.Remove Widget Under Water` _asbp_player_character))

(event `self.ReceiveTick`
  (params (DeltaSeconds :type "Float (single-precision)"))
  (bind (_returnvalue_x _returnvalue_y _returnvalue_z) (`KismetMathLibrary.BreakVector` (`SceneComponent.K2_GetComponentScale` (`self.StaticMesh`))))
  (bind _returnvalue (+ _returnvalue_z (/ (* DeltaSeconds (`self.Nums of Holes`)) 10.0)))
  (if (<= _returnvalue 0.0)
    (set `self.Scale Z` 0.0)
    (else
      (set `self.Scale Z` _returnvalue)))
  (`SceneComponent.SetWorldScale3D` (`self.StaticMesh`) (`KismetMathLibrary.MakeVector` _returnvalue_x _returnvalue_y (`self.Scale Z`))))

(fn `Change Nims of Holes`
  (params (`Increase?` :type Boolean))
  (if `Increase?`
    (`/Engine/EditorBlueprintResources/StandardMacros.IncrementInt` (`self.Nums of Holes`))
    (else
      (`/Engine/EditorBlueprintResources/StandardMacros.DecrementInt` (`self.Nums of Holes`)))))

(fn `Decrease Water Level`
  (locals (`Water Speed` :type "Float (double-precision)" :default 10.0))
  (bind (_returnvalue_x _returnvalue_y _returnvalue_z) (`KismetMathLibrary.BreakVector` (`SceneComponent.K2_GetComponentScale` (`self.StaticMesh`))))
  (for _index (range 11)
    (bind _returnvalue (- _returnvalue_z (/ _index (`local.Water Speed`))))
    (if (<= _returnvalue 0.0)
      (`SceneComponent.SetWorldScale3D` (`self.StaticMesh`) (`KismetMathLibrary.MakeVector` _returnvalue_x _returnvalue_y))
      (else
        (`SceneComponent.SetWorldScale3D` (`self.StaticMesh`) (`KismetMathLibrary.MakeVector` _returnvalue_x _returnvalue_y _returnvalue))))))

(fn `UserConstructionScript`)