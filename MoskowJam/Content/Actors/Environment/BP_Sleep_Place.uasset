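; Sleep place work station where bots that are sent to relax play a relax animation.
; On begin play it sets its animation and required worker tags, then activates the work station.
; When an overlapping bot carries the required tag, it disables interaction collision, adds the animation tag, then after a fixed delay removes it and re-enables collision.
; Tags are exchanged through message calls; a node to align bot rotation is left unconnected.
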(event `self.ReceiveBeginPlay`
  (`parent.ReceiveBeginPlay`)
  (set `self.ThisWorkAnim` (struct :`TagName` "Anim.Relax.#1"))
  (set `self.ThisWorkerTagReq` (struct :`TagName` "Go.ToRelax.Place1"))
  (message `/Game/Interfaces/IBP_HR.Activate WorkStation` self))

(event `self.Interaction.OnComponentBeginOverlap`
  (params (OverlappedComponent :type "PrimitiveComponent Object Reference") (OtherActor :type "Actor Object Reference") (OtherComp :type "PrimitiveComponent Object Reference") (OtherBodyIndex :type Integer) (bFromSweep :type Boolean) (SweepResult :type "HitResult Structure (by ref)"))
  (set `self.Bot` OtherActor)
  ;[1 1 1] Если этот бот идёт сюда (имеет нужный нам тэг)
  (bind _has (message `/Game/Interfaces/IBP_Tags_Management.Has Tag` (`self.Bot`) (`self.ThisWorkerTagReq`) false))
  (if _has
    (`PrimitiveComponent.SetCollisionEnabled` (`self.Interaction`) "NoCollision")
    ;[1 1 1] То мы даём ему тег анимации этой работы
    (message `/Game/Interfaces/IBP_Tags_Management.Add Tag` (`self.Bot`) (`self.ThisWorkAnim`))
    (`KismetSystemLibrary.Delay` 10.0)
    (message `/Game/Interfaces/IBP_Tags_Management.Remove Tag` (`self.Bot`) (`self.ThisWorkAnim`))
    (`PrimitiveComponent.SetCollisionEnabled` (`self.Interaction`) "QueryOnly")))

(fn `UserConstructionScript`
  (`parent.UserConstructionScript`))