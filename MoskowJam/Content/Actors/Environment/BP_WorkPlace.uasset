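; Configurable submarine crew workstation (engine, wheel, torpedoes, rest spots), with an enum selecting its gameplay tags, mesh and AnimBP.
; An overlapping bot carrying the required tag locks the station, receives a work animation tag and, after a delay, triggers WorkResult.
; WorkResult switches on the bot's task tag to drive BP_Submarine speed, dodges and torpedoes, chaining rearm to the SetTorpedos station.
; GetSubTask maps orders to task tags with stamina and stress costs.
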(event `self.ReceiveBeginPlay`
  (bind _thisworkstation (`self.ThisWorkStation`))
  ;[1 1 1] В зависимости от типа станции, задаём вторичные игровые теги: какого работника ищем, какой тег анимации передаём
  (`parent.ReceiveBeginPlay`)
  (`self.ChooseSecondaryTags` _thisworkstation)
  ;[1 1 1] Помечаем этого актора тегом с названием станка
  (bind _output_get (set `self.TagName` (`|GetEnumeratorNameAsString` _thisworkstation)))
  (set `self.Tags` (`|MakeArray` (`KismetStringLibrary.Conv_StringToName` _output_get)))
  (`KismetSystemLibrary.DrawDebugString` (`self.K2_GetActorLocation` self) _output_get null (struct :`R` 0.166667 :`G` 0.007619 :`B` 0.004303 :`A` 1.0) 300.0)
  (if (`self.Activated on Start`)
    ;[1 1 1] На старте активно
    (`PrimitiveComponent.SetCollisionEnabled` (`self.Interaction`) "QueryOnly")
    (else
      ;[1 1 1] На старте не предлагает работу
      (`PrimitiveComponent.SetCollisionEnabled` (`self.Interaction`) "NoCollision"))))

(event `/Game/Interfaces/IBP_HR.Activate WorkStation`
  ;[1 1 1] Если нужно что-то сделать на этой установке, отправляем сигнал, чтобы установка начала работать
  (`PrimitiveComponent.SetCollisionEnabled` (`self.Interaction`) "QueryOnly")
  (`KismetSystemLibrary.PrintString` "Активировано" true true (struct :`R` 0.023316 :`G` 0.101317 :`B` 1.0 :`A` 1.0) 20.0))

(event `self.ReceiveActorBeginOverlap`
  (params (OtherActor :type "Actor Object Reference"))
  (`parent.ReceiveActorBeginOverlap` null))

(event `self.Interaction.OnComponentBeginOverlap`
  (params (OverlappedComponent :type "PrimitiveComponent Object Reference") (OtherActor :type "Actor Object Reference") (OtherComp :type "PrimitiveComponent Object Reference") (OtherBodyIndex :type Integer) (bFromSweep :type Boolean) (SweepResult :type "HitResult Structure (by ref)"))
  (set `self.Bot` OtherActor)
  ;[1 1 1] Если этот бот идёт сюда (имеет нужный нам тэг)
  (bind _has (message `/Game/Interfaces/IBP_Tags_Management.Has Tag` (`self.Bot`) (`self.ThisWorkerTagReq`) false))
  (if _has
    ;[1 1 1] Отключаем коллизию, чтобы повторно кого-нибудь  не назначить на эту работу
    (`PrimitiveComponent.SetCollisionEnabled` (`self.Interaction`) "NoCollision")
    ;[1 1 1] То мы даём ему тег анимации этой работы
    (bind _added (message `/Game/Interfaces/IBP_Tags_Management.Add Tag` (`self.Bot`) (`self.ThisWorkAnim`)))
    (if _added
      (`self.K2_SetActorRotation` (`self.Bot`) (`self.K2_GetActorRotation` self) false)
      ;[1 1 1] Даём какое-то время на работу
      (`KismetSystemLibrary.Delay` (`self.DurationOfProccess`))
      ;[1 1 1] Определяем результат работы по тегу работника
      (bind _work_tag (message `/Game/Interfaces/IBP_Tags_Management.Get Work Tag` (`self.Bot`)))
      (`self.Work Result` _work_tag)
      (`KismetSystemLibrary.Delay` (`self.Duration_Of_Animation`))
      ;[1 1 1] Удаляем тег этой анимации у работника
      (`self.This worker finished his work` (`self.Bot`) (`self.ThisWorkAnim`))
      ;[1 1 1] После окончания процесса удаляем тег у этого актора и больше не ищем ему работников
      (`BlueprintGameplayTagLibrary.RemoveGameplayTag` (`self.Tag Container`) (struct :`TagName` "Workstation.InProgress"))
      (`KismetSystemLibrary.PrintString` "Деактивировано" true true (struct :`R` 0.006934 :`G` 1.0 :`A` 1.0) 20.0))))

(event `self.ReceiveTick`
  (params (DeltaSeconds :type "Float (single-precision)"))
  (`KismetSystemLibrary.PrintString` (`KismetStringLibrary.Concat_StrStr` (`self.TagName`) " 1: " (`KismetStringLibrary.Conv_BoolToString` (`self.Anim_State_1`)) " 2:" (`KismetStringLibrary.Conv_BoolToString` (`self.Anim_State_2`)) " 3: " (`KismetStringLibrary.Conv_BoolToString` (`self.Anim_State_3`))) true true (struct :`R` 1.0 :`G` 0.116777 :`B` 0.186486 :`A` 1.0) 0.0))

(event `/Game/Interfaces/IBP_HR.Set INPROGRESS`
  ;[1 1 1] Если к станции вышел сотрудник, то она занята
  (`BlueprintGameplayTagLibrary.AddGameplayTag` (`self.Tag Container`) (struct :`TagName` "Workstation.InProgress")))

(fn `Add Tag`
  (params (`Add Tag` :type "GameplayTag Structure")))

(fn `Choose Skeletal Mesh and Animation`
  (params (Selection :type "/Game/Enums/EWorkStations Enum" :default "NewEnumerator0"))
  (switch `/Game/Enums/EWorkStations` Selection
    (:`NewEnumerator0`
      (`SkeletalMeshComponent.SetSkeletalMeshAsset` (`self.SkeletalMesh`) "/Game/ART/Engine/engine.engine")
      (`SkeletalMeshComponent.SetAnimInstanceClass` (`self.SkeletalMesh`) "/Game/ART/AnimCharact/Engine/Animations/ABP_Engine.ABP_Engine_C"))
    (:`NewEnumerator1`
      (`SkeletalMeshComponent.SetSkeletalMeshAsset` (`self.SkeletalMesh`) "/Game/ART/rull/Rull.Rull")
      (`SkeletalMeshComponent.SetAnimInstanceClass` (`self.SkeletalMesh`) "/Game/ART/AnimCharact/Wheel/Animations/ABP_Rull.ABP_Rull_C"))
    (:`NewEnumerator2`
      (`SkeletalMeshComponent.SetSkeletalMeshAsset` (`self.SkeletalMesh`) null :!label _label)
      (`SkeletalMeshComponent.SetAnimInstanceClass` (`self.SkeletalMesh`) null))
    (:`NewEnumerator3`
      (goto _label))
    (:`NewEnumerator4`
      (goto _label))
    (:`NewEnumerator5`
      (goto _label))
    (:`NewEnumerator6`
      (goto _label))
    (:`NewEnumerator7`
      (goto _label))))

(fn `ChooseSecondaryTags`
  (params (`This Work Station` :type "/Game/Enums/EWorkStations Enum" :default "NewEnumerator0"))
  (switch `/Game/Enums/EWorkStations` `This Work Station`
    (:`NewEnumerator0`
      (set `self.ThisWorkerTagReq` (struct :`TagName` "Go.ToWork.Engine"))
      (set `self.ThisWorkAnim` (struct :`TagName` "Anim.Working.Engine"))
      (`BlueprintGameplayTagLibrary.AddGameplayTag` (`self.SubTask Anim`) (struct :`TagName` "Anim.Working.Engine.FullForward"))
      (`BlueprintGameplayTagLibrary.AddGameplayTag` (`self.SubTask Anim`) (struct :`TagName` "Anim.Working.Engine.HalfForward"))
      (`BlueprintGameplayTagLibrary.AddGameplayTag` (`self.SubTask Anim`) (struct :`TagName` "Anim.Working.Engine.Stop"))
      (`BlueprintGameplayTagLibrary.AddGameplayTag` (`self.SubTask Tags`) (struct :`TagName` "Go.ToWork.Engine.FullForward"))
      (`BlueprintGameplayTagLibrary.AddGameplayTag` (`self.SubTask Tags`) (struct :`TagName` "Go.ToWork.Engine.HalfForward"))
      (`BlueprintGameplayTagLibrary.AddGameplayTag` (`self.SubTask Tags`) (struct :`TagName` "Go.ToWork.Engine.FullForward")))
    (:`NewEnumerator1`
      (set `self.ThisWorkerTagReq` (struct :`TagName` "Go.ToWork.Wheel"))
      (set `self.ThisWorkAnim` (struct :`TagName` "Anim.Working.Wheel"))
      (`BlueprintGameplayTagLibrary.AddGameplayTag` (`self.SubTask Anim`) (struct :`TagName` "Anim.Working.Wheel.Right"))
      (`BlueprintGameplayTagLibrary.AddGameplayTag` (`self.SubTask Anim`) (struct :`TagName` "Anim.Working.Wheel.Left"))
      (`BlueprintGameplayTagLibrary.AddGameplayTag` (`self.SubTask Tags`) (struct :`TagName` "Go.ToWork.Wheel.Right"))
      (`BlueprintGameplayTagLibrary.AddGameplayTag` (`self.SubTask Tags`) (struct :`TagName` "Go.ToWork.Wheel.Left")))
    (:`NewEnumerator2`
      (set `self.ThisWorkerTagReq` (struct :`TagName` "Go.ToWork.Torpedos"))
      (set `self.ThisWorkAnim` (struct :`TagName` "Anim.Working.Torpedos"))
      (`BlueprintGameplayTagLibrary.AddGameplayTag` (`self.SubTask Anim`) (struct :`TagName` "Anim.Working.Torpedos.Fire"))
      (`BlueprintGameplayTagLibrary.AddGameplayTag` (`self.SubTask Anim`) (struct :`TagName` "Anim.Working.Torpedos.Rearm"))
      (`BlueprintGameplayTagLibrary.AddGameplayTag` (`self.SubTask Tags`) (struct :`TagName` "Go.ToWork.Torpedos.Rearm"))
      (`BlueprintGameplayTagLibrary.AddGameplayTag` (`self.SubTask Tags`) (struct :`TagName` "Go.ToWork.Torpedos.Fire")))
    (:`NewEnumerator3`
      (set `self.ThisWorkerTagReq` (struct :`TagName` "Go.ToRelax.Place1"))
      (set `self.ThisWorkAnim` (struct :`TagName` "Anim.Relax.#1")))
    (:`NewEnumerator4`
      (set `self.ThisWorkerTagReq` (struct :`TagName` "Go.ToRelax.Place2"))
      (set `self.ThisWorkAnim` (struct :`TagName` "Anim.Relax.#2")))
    (:`NewEnumerator5`
      (set `self.ThisWorkerTagReq` (struct :`TagName` "Go.ToRelax.Place3"))
      (set `self.ThisWorkAnim` (struct :`TagName` "Anim.Relax.#3")))
    (:`NewEnumerator6`
      (set `self.ThisWorkerTagReq` (struct :`TagName` "Go.ToWork.Torpedos"))
      (set `self.ThisWorkAnim` (struct :`TagName` "Anim.Working.Torpedos.Rearm.GetMissle")))
    (:`NewEnumerator7`
      (set `self.ThisWorkerTagReq` (struct :`TagName` "Go.ToWork.Torpedos"))
      (set `self.ThisWorkAnim` (struct :`TagName` "Anim.Working.Torpedos.Rearm.SetMissle")))))

(fn `Get Anim Tag`
  (returns (`Anim Tag` :type "GameplayTag Structure"))
  (return))

(fn `Get SubTask`
  (params (SubTask :type "/Game/Enums/EButtonSubtypes Enum" :default "NewEnumerator0"))
  (returns (`SubTask Tag` :type "GameplayTag Structure") (`Add to Stress` :type "Float (double-precision)") (`Stamina Damage Value` :type "Float (double-precision)"))
  (locals (`Stamina Damage` :type "Float (double-precision)") (`Stress Add` :type "Float (double-precision)"))
  (switch `/Game/Enums/EButtonSubtypes` SubTask
    (:`NewEnumerator0`
      (bind _output_get (set `local.Stamina Damage` 20.0))
      (bind _output_get_2 (set `local.Stress Add` 5.0))
      (return (struct :`TagName` "Go.ToWork.Wheel.Right") _output_get_2 _output_get))
    (:`NewEnumerator1`
      (bind _output_get_3 (set `local.Stamina Damage` 20.0))
      (bind _output_get_4 (set `local.Stress Add` 5.0))
      (return (struct :`TagName` "Go.ToWork.Wheel.Left") _output_get_4 _output_get_3))
    (:`NewEnumerator2`
      (bind _output_get_5 (set `local.Stamina Damage` 30.0))
      (bind _output_get_6 (set `local.Stress Add` 15.0))
      (return (struct :`TagName` "Go.ToWork.Engine.FullForward") _output_get_6 _output_get_5))
    (:`NewEnumerator3`
      (bind _output_get_7 (set `local.Stamina Damage` 15.0))
      (bind _output_get_8 (set `local.Stress Add` 10.0))
      (return (struct :`TagName` "Go.ToWork.Engine.HalfForward") _output_get_8 _output_get_7))
    (:`NewEnumerator8`
      (bind _output_get_9 (set `local.Stamina Damage` 5.0))
      (bind _output_get_10 (set `local.Stress Add` 5.0))
      (return (struct :`TagName` "Go.ToWork.Engine.StopMachine") _output_get_10 _output_get_9))
    (:`NewEnumerator4`
      (set `local.Stamina Damage` 0.0)
      (set `local.Stress Add` -30.0))
    (:`NewEnumerator5`
      (bind _output_get_11 (set `local.Stamina Damage` 0.0))
      (bind _output_get_12 (set `local.Stress Add` 1.0))
      (return (struct :`TagName` "Go.ToRelax.Place1") _output_get_12 _output_get_11))
    (:`NewEnumerator6`
      (bind _output_get_13 (set `local.Stamina Damage` 40.0))
      (bind _output_get_14 (set `local.Stress Add` 20.0))
      (return (struct :`TagName` "Go.ToWork.Torpedos.Rearm") _output_get_14 _output_get_13))
    (:`NewEnumerator7`
      (bind _output_get_15 (set `local.Stamina Damage` 10.0))
      (bind _output_get_16 (set `local.Stress Add` 10.0))
      (return (struct :`TagName` "Go.ToWork.Torpedos.Fire") _output_get_16 _output_get_15))))

(fn `Get This Worker Req Tag`
  (returns (ThisWorkerTagReq :type "GameplayTag Structure"))
  (return (`self.ThisWorkerTagReq`)))

(fn `Get Work Tag`
  (returns (`Work Tag` :type "GameplayTag Structure"))
  (return))

(fn `Has Tag`
  (params (`Has Tag` :type "GameplayTag Structure") (`Exect Match` :type Boolean))
  (returns (Has :type Boolean))
  (return (`BlueprintGameplayTagLibrary.MatchesAnyTags` `Has Tag` (`self.Tag Container`) `Exect Match`)))

(fn `Remove Tag`
  (params (`Remove Tag` :type "GameplayTag Structure")))

(fn `Set State Animation`
  (params (Anim_State_1 :type Boolean) (Anim_State_2 :type Boolean) (Anim_State_3 :type Boolean))
  (if Anim_State_1
    (set `self.Anim_State_1` true)
    (set `self.Anim_State_2` false)
    (set `self.Anim_State_3` false)
    (elif Anim_State_2
      (set `self.Anim_State_1` false)
      (set `self.Anim_State_2` true)
      (set `self.Anim_State_3` false)
      (else
        (set `self.Anim_State_1` false)
        (set `self.Anim_State_2` false)
        (set `self.Anim_State_3` true)))))

(fn `UserConstructionScript`
  (`parent.UserConstructionScript`)
  (`self.Choose Skeletal Mesh and Animation` (`self.ThisWorkStation`))
  (`SceneComponent.SetWorldScale3D` (`self.SkeletalMesh`) (`self.New Scale`))
  (`SceneComponent.K2_SetWorldLocationAndRotation` (`self.SkeletalMesh`) (`self.New Location`) (`self.New Rotation`) false false))

(fn `Work Result`
  (params (`SubTastk Tag` :type "GameplayTag Structure"))
  (locals (`Local Submarin` :type "Submarine Object Reference") (`Delta Speed Max` :type "Float (single-precision)" :default 1000.0) (`Delta Speed Half` :type "Float (single-precision)" :default 500.0) (`Null Speed` :type "Float (single-precision)" :default 0.0) (`Local BP_Submarine` :type "/Game/Test/BP_Submarine Object Reference") (`Local Set Torpedos` :type "/Game/Actors/Environment/BP_WorkPlace Object Reference"))
  (bind _delta_speed_max (`local.Delta Speed Max`))
  (bind _delta_speed_half (`local.Delta Speed Half`))
  (bind _null_speed (`local.Null Speed`))
  ;[1 1 1] Эта гидра решает, какая функция должна выполняться в зависимости от имеющейся задачи
  (bind _returnvalue (`/Game/Library/FL_General.Get Submarine`))
  (bind _output_get (set `local.Local Submarin` _returnvalue))
  (bind _asbp_submarine (cast `/Game/Test/BP_Submarine` _output_get))
  (set `local.Local BP_Submarine` _asbp_submarine)
  (`|SwitchGameplayTag` `SubTastk Tag`
    (:`Go.ToWork.Engine.FullForward`
      (`KismetSystemLibrary.PrintString` "Полный ход!")
      (`Submarine.Set_CurrentSpeed` (`local.Local BP_Submarine`) _delta_speed_max)
      (`KismetSystemLibrary.PrintString` (`KismetStringLibrary.Conv_DoubleToString` _delta_speed_max))
      (message `/Game/Interfaces/IBP_Tags_Management.Add Tag` (`self.Bot`) (struct :`TagName` "Anim.Working.Engine.FullForward"))
      (message `/Game/Interfaces/IBP_HR.Work Result Message` (`self.Bot`) "Полный ход работает на полную!")
      (`self.Set State Animation` false false true))
    (:`Go.ToWork.Engine.HalfForward`
      (`KismetSystemLibrary.PrintString` "Неполный ход!")
      (`Submarine.Set_CurrentSpeed` (`local.Local BP_Submarine`) _delta_speed_half)
      (`KismetSystemLibrary.PrintString` (`KismetStringLibrary.Conv_DoubleToString` _delta_speed_half))
      (message `/Game/Interfaces/IBP_Tags_Management.Add Tag` (`self.Bot`) (struct :`TagName` "Anim.Working.Engine.HalfForward"))
      (message `/Game/Interfaces/IBP_HR.Work Result Message` (`self.Bot`) "Неполный ход работает на неполную!")
      (`self.Set State Animation` false true))
    (:`Go.ToWork.Engine.StopMachine`
      (`KismetSystemLibrary.PrintString` "Стоп Машина!")
      (`Submarine.Set_CurrentSpeed` (`local.Local BP_Submarine`) _null_speed)
      (`KismetSystemLibrary.PrintString` (`KismetStringLibrary.Conv_DoubleToString` _null_speed))
      (message `/Game/Interfaces/IBP_Tags_Management.Add Tag` (`self.Bot`) (struct :`TagName` "Anim.Working.Engine.Stop"))
      (message `/Game/Interfaces/IBP_HR.Work Result Message` (`self.Bot`) "Двигатель заглушен")
      (`self.Set State Animation` true))
    (:`Go.ToWork.Torpedos.Fire`
      (`KismetSystemLibrary.PrintString` "Submarine loaded?")
      (bind _missle_armed (`/Game/Test/BP_Submarine.Get is Missle Armed` (`local.Local BP_Submarine`)))
      (if _missle_armed
        (`KismetSystemLibrary.PrintString` "Пли!")
        (`/Game/Test/BP_Submarine.Spawn Missle` (`local.Local BP_Submarine`))
        (message `/Game/Interfaces/IBP_HR.Work Result Message` (`self.Bot`) "Торпеда пошла!")
        (else
          (`KismetSystemLibrary.PrintString` "Нужно зарядить!")
          (message `/Game/Interfaces/IBP_HR.Work Result Message` (`self.Bot`) "Не могу, орудие не заряжено!"))))
    (:`Go.ToWork.Torpedos.Rearm`
      (`KismetSystemLibrary.PrintString` "Submarine loaded?")
      (bind _missle_armed_2 (`/Game/Test/BP_Submarine.Get is Missle Armed` (`local.Local BP_Submarine`)))
      (if _missle_armed_2
        (`KismetSystemLibrary.PrintString` "Не надо перезаряжать!")
        (message `/Game/Interfaces/IBP_HR.Work Result Message` (`self.Bot`) "Не могу, орудие уже заряжено")
        (elif (`self.Second Phase`)
          (`/Game/Test/BP_Submarine.Set is Missle Armed` (`local.Local BP_Submarine`) true)
          (message `/Game/Interfaces/IBP_HR.Work Result Message` (`self.Bot`) "Перезарядил!")
          (else
            (`KismetSystemLibrary.PrintString` "Перезарядить!")
            (message `/Game/Interfaces/IBP_Tags_Management.Add Tag` (`self.Bot`) (struct :`TagName` "Anim.Working.Torpedos.Rearm.GetMissle"))
            (bind _asbp_sailor (cast `/Game/Actors/Bots/BP_Sailor` (`self.Bot`)))
            (`/Game/Actors/Bots/BP_Sailor. Set Have Torpedos` _asbp_sailor true)
            (bind _outactors (`GameplayStatics.GetAllActorsOfClassWithTag` "BP_WorkPlace_C" "SetTorpedos"))
            (for _array_element _outactors
              (set `local.Local Set Torpedos` _array_element))
            (`/Game/Actors/Bots/BP_Sailor.Set PlaceToWork` _asbp_sailor (`local.Local Set Torpedos`))
            (`/Game/Interfaces/IBP_HR.Activate WorkStation` (`local.Local Set Torpedos`))))))
    (:`Go.ToWork.Wheel.Left`
      (`KismetSystemLibrary.PrintString` "Лево Руля!")
      (`Submarine.StartManeuver_Dodge` (`local.Local Submarin`) "Left")
      (message `/Game/Interfaces/IBP_Tags_Management.Add Tag` (`self.Bot`) (struct :`TagName` "Anim.Working.Wheel.Left"))
      (message `/Game/Interfaces/IBP_HR.Work Result Message` (`self.Bot`) "Сместились налево!")
      (`self.Set State Animation` false false true))
    (:`Go.ToWork.Wheel.Right`
      (`KismetSystemLibrary.PrintString` "Право Руля")
      (`Submarine.StartManeuver_Dodge` (`local.Local Submarin`) "Right")
      (message `/Game/Interfaces/IBP_Tags_Management.Add Tag` (`self.Bot`) (struct :`TagName` "Anim.Working.Wheel.Right"))
      (message `/Game/Interfaces/IBP_HR.Work Result Message` (`self.Bot`) "Сместились направо!")
      (`self.Set State Animation` false true))
    (:`Go.ToRelax.Place1`
      (message `/Game/Interfaces/IBP_Tags_Management.Add Tag` (`self.Bot`) (struct :`TagName` "Anim.Relax.#1"))
      (`/Game/Interfaces/IBP_HR.Activate WorkStation` self))
    (:`Go.ToRelax.Place2`
      (message `/Game/Interfaces/IBP_Tags_Management.Add Tag` (`self.Bot`) (struct :`TagName` "Anim.Relax.#2"))
      (`/Game/Interfaces/IBP_HR.Activate WorkStation` self))))