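; NPC manager that assigns work to sailor cats (BP_Cat_Sailor) and tracks which are free.
; SetWorkTask picks the free cat with most stamina, charges stamina and stress, then tags it and activates the workplace.
; Workplace finish callbacks remove the tag and return the cat to the free list.
; BeginPlay also starts looping timers meant for rest recovery; SetCatToWork and the manager's own DamageStamina are stubs.
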(event `self.ReceiveBeginPlay`
  ;[1 1 1] Создаём массив котиков и массив неработающих котиков. В начале иигры они равны
  (bind _outactors (`GameplayStatics.GetAllActorsOfClass` "/Game/Actors/Bots/BP_Cat_Sailor.BP_Cat_Sailor_C"))
  (bind _output_get (set `self.Array of Cats` _outactors))
  (set `self.Array of Free Cats` _output_get)
  ;[1 1 1] Подписываемся к каждому котику на завершение им его работы. Если котик завершил работу, то возвращаем его в список неработающих котиков
  (bind _outactors_2 (`GameplayStatics.GetAllActorsOfClass` "/Game/Actors/Environment/BP_WorkPlace.BP_WorkPlace_C"))
  (for _array_element _outactors_2
    (add `/Game/Actors/Environment/BP_WorkPlace.This worker finished his work` _array_element (delegate `This Worker Finished his work Helper`))
    ;[1 1 1] По таймеру регенирируем отдыхающим котикам стамину и стресс
    (bind _asbp_game_mode_base_mj (`/Game/Library/FL_General.Get MJ GameMode`))
    (`KismetSystemLibrary.K2_SetTimerDelegate` (`|CreateDelegate` _asbp_game_mode_base_mj :!event `Regen Stamina`) (`self.Relax#1 Timer`) true true)))

(event `This Worker Finished his work Helper`
  (params (`This worker` :type "Actor Object Reference") (`Tag to Remove` :type "GameplayTag Structure"))
  ;[1 1 1] Подписываемся к каждому котику на завершение им его работы. Если котик завершил работу, то возвращаем его в список неработающих котиков
  (bind _asbp_cat_sailor (cast `/Game/Actors/Bots/BP_Cat_Sailor` `This worker`))
  (message `/Game/Interfaces/IBP_Tags_Management.Remove Tag` _asbp_cat_sailor `Tag to Remove`)
  (`KismetArrayLibrary.Array_AddUnique` (`self.Array of Free Cats`) _asbp_cat_sailor))

(fn `Damage Stamina`
  (params (`Damage Stamina` :type "Float (double-precision)"))
  (returns (`Not Enought` :type Boolean))
  (return false))

(fn `Find NPC in Array with Max Stamina`
  (params (`Input array of NPC` :type "Array of /Game/Actors/Bots/BP_Cat_Sailor Object Reference"))
  (returns (`This one Have max stamina` :type "/Game/Actors/Bots/BP_Cat_Sailor Object Reference"))
  (locals (`Local Array of Float` :type "Array of Float (double-precision)") (`Have max stamina` :type "/Game/Actors/Bots/BP_Cat_Sailor Object Reference") (`Local Array of Free Cats` :type "Array of /Game/Actors/Bots/BP_Cat_Sailor Object Reference"))
  (bind _output_get (set `local.Local Array of Free Cats` `Input array of NPC`))
  (for _array_element _output_get
    (bind _scale_stamina (`/Game/Actors/Bots/BP_Sailor.Get Scale Stamina Component` _array_element))
    (bind _current (`/Game/Components/CBP_Scale.Get Current` _scale_stamina))
    (`KismetArrayLibrary.Array_Add` (`local.Local Array of Float`) _current))
  (bind (_return_max _return_index_of_max) (`self.Max in Array of Float` (`local.Local Array of Float`)))
  (for (_array_element_2 _array_index) (`local.Local Array of Free Cats`)
    (if (== _array_index _return_index_of_max)
      (set `local.Have max stamina` _array_element_2)))
  (return (`local.Have max stamina`)))

(fn `Get Array of Cats`
  (returns (`Array of Cats` :type "Array of /Game/Actors/Bots/BP_Cat_Sailor Object Reference"))
  (return (`self.Array of Cats`)))

(fn `Get Array of Free Cats`
  (returns (`Array of Free Cats` :type "Array of /Game/Actors/Bots/BP_Cat_Sailor Object Reference"))
  (return (`self.Array of Free Cats`)))

(fn `Max in Array of Float`
  (params (InterFloat :type "Array of Float (double-precision)"))
  (returns (`Return Max` :type "Float (double-precision)") (`Return index of max` :type Integer))
  (locals (`length of array` :type Integer :default 0) (`Local Array` :type "Array of Float (double-precision)") (Max :type "Float (double-precision)") (`index of max` :type Integer))
  (bind _output_get (set `local.Local Array` InterFloat))
  (bind _output_get_2 (set `local.length of array` (`KismetArrayLibrary.Array_Length` _output_get)))
  (if (> _output_get_2 0)
    (set `local.Max` (`|GetArrayItem` (`local.Local Array`)))
    (set `local.index of max` 0)
    (for _index (range 1 (`local.length of array`))
      (bind _output (`|GetArrayItem` (`local.Local Array`) _index))
      (if (> _output (`local.Max`))
        (set `local.Max` _output)
        (set `local.index of max` _index)))
    (return (`local.Max`) (`local.index of max`))))

(fn `Set Cat to Work`)

(fn `Set Work Task`
  (params (ThisPlace :type "Object Object Reference") (ThisWorkReqTag :type "GameplayTag Structure") (`Stamina Cost` :type "Float (double-precision)") (`Stress Cost` :type "Float (double-precision)"))
  (returns (`Work set` :type Boolean))
  (locals (`Local This Place` :type "Object Object Reference") (`Local Req Tag` :type "GameplayTag Structure") (`Local This One` :type "/Game/Actors/Bots/BP_Cat_Sailor Object Reference") (`Local Stamina Cost` :type "Float (double-precision)") (`Local Stress Cost` :type "Float (double-precision)"))
  (set `local.Local This Place` ThisPlace)
  (set `local.Local Req Tag` ThisWorkReqTag)
  (set `local.Local Stamina Cost` `Stamina Cost`)
  (set `local.Local Stress Cost` `Stress Cost`)
  (bind _this_one_have_max_stamina (`self.Find NPC in Array with Max Stamina` (`self.Array of Free Cats`)))
  (bind _output_get (set `local.Local This One` _this_one_have_max_stamina))
  (bind _not_enought (`/Game/Actors/Bots/BP_Sailor.Damage Stamina` _output_get (`local.Local Stamina Cost`)))
  (if _not_enought
    (`/Game/Actors/Bots/BP_Sailor.Increase Stress` (`local.Local This One`) (`local.Local Stress Cost`))
    (message `/Game/Interfaces/IBP_HR.Activate WorkStation` (`local.Local This Place`))
    (`/Game/Actors/Bots/BP_Sailor.Set PlaceToWork` (`local.Local This One`) (`local.Local This Place`))
    (bind _added (message `/Game/Interfaces/IBP_Tags_Management.Add Tag` (`local.Local This One`) (`local.Local Req Tag`)))
    (if _added
      (`KismetArrayLibrary.Array_RemoveItem` (`self.Array of Free Cats`) (`local.Local This One`))
      (message `/Game/Interfaces/IBP_HR.Set INPROGRESS` (`local.Local This Place`)))
    (return _added)
    (else
      (return _not_enought))))

(fn `UserConstructionScript`)