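; Interactable environment panel that opens the Commander Panel UI when the player presses E nearby.
; A box trigger detects the tagged player capsule, stores the actor as Commander, shows an interaction prompt and adds the interaction-zone input mapping context.
; The player controller's E-press event rechecks the overlap, then creates the panel widget from button data, sets Commander as owner and clears the prompt and mapping, as does leaving the box.
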(event `self.Box.OnComponentBeginOverlap`
  (params (OverlappedComponent :type "PrimitiveComponent Object Reference") (OtherActor :type "Actor Object Reference") (OtherComp :type "PrimitiveComponent Object Reference") (OtherBodyIndex :type Integer) (bFromSweep :type Boolean) (SweepResult :type "HitResult Structure (by ref)"))
  (if (`ActorComponent.ComponentHasTag` OtherComp "Player Capsule")
    (set `self.Commander` OtherActor)
    (bind _interaction (`/Game/Library/FL_General.Create Interaction Widget` "Взаимодействовать"))
    (set `self.Interaction` _interaction)
    (message `EnhancedInputSubsystemInterface.AddMappingContext` (`GameplayStatics.GetPlayerController` 0) "/Game/GameSettings/IMC_Interaction_Zone.IMC_Interaction_Zone" 0 (struct))))

(event `self.Box.OnComponentEndOverlap`
  (params (OverlappedComponent :type "PrimitiveComponent Object Reference") (OtherActor :type "Actor Object Reference") (OtherComp :type "PrimitiveComponent Object Reference") (OtherBodyIndex :type Integer))
  (if (`ActorComponent.ComponentHasTag` OtherComp "Player Capsule")
    (`self.Close Interaction Widget`)))

(event `self.ReceiveBeginPlay`
  (bind _asbp_player_controller_mj (cast `/Game/GameSettings/BP_PlayerController_MJ` (`GameplayStatics.GetPlayerController` 0)))
  (add `/Game/GameSettings/BP_PlayerController_MJ.E pressed` _asbp_player_controller_mj (delegate `E pressed Helper`)))

(event `E pressed Helper`
  (for _array_element (`PrimitiveComponent.GetOverlappingComponents` (`self.Box`))
    (if (`ActorComponent.ComponentHasTag` _array_element "Player Capsule")
      (bind _command_panel (`/Game/Library/FL_General.Create Commander Panel` 0 (`self.Array Of Buttons Data`) true))
      (bind _output_get (set `self.Commander Panel` _command_panel))
      (`/Game/GUI/BPW_CommanderMenu.Set Owner` _output_get (`self.Commander`))
      (`self.Close Interaction Widget`))))

(fn `Close Interaction Widget`
  (`/Engine/EditorBlueprintResources/StandardMacros.IsValid` (`self.Interaction`)
    (:`Is Valid`
      (`Widget.RemoveFromParent` (`self.Interaction`)))
    (:`Is Not Valid`
      _))
  (message `EnhancedInputSubsystemInterface.RemoveMappingContext` (`GameplayStatics.GetPlayerController` 0) "/Game/GameSettings/IMC_Interaction_Zone.IMC_Interaction_Zone" (struct)))

(fn `UserConstructionScript`)