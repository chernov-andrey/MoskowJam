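; BP_Decoration is an environment decoration actor that randomizes its stone appearance when play begins.
; A random boolean on BeginPlay assigns either the Stone2 mesh or the Stone3 mesh, with the Stone3 variant also scaled up fivefold.
; Every Tick, an Arrow component is rotated in world space to point along MoveDirection, though nothing in these graphs moves the actor.
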(event `self.ReceiveBeginPlay`
  (bind _staticmeshcomponent (`self.StaticMeshComponent`))
  (bind _staticmeshcomponent_2 (`self.StaticMeshComponent`))
  (if (`KismetMathLibrary.RandomBool`)
    (`StaticMeshComponent.SetStaticMesh` _staticmeshcomponent (select `bool` false :`false` "/Game/Actors/Environment/Models/stone2.stone2" :`true` "/Game/Actors/Environment/Models/stone3.stone3" :!type "StaticMesh Object Reference"))
    (else
      (`SceneComponent.SetRelativeScale3D` _staticmeshcomponent_2 (* (`SceneComponent.K2_GetComponentScale` _staticmeshcomponent_2) 5.0))
      (`StaticMeshComponent.SetStaticMesh` _staticmeshcomponent (select `bool` true :`false` "/Game/Actors/Environment/Models/stone2.stone2" :`true` "/Game/Actors/Environment/Models/stone3.stone3" :!type "StaticMesh Object Reference")))))

(event `self.ReceiveTick`
  (params (DeltaSeconds :type "Float (single-precision)"))
  (`SceneComponent.K2_SetWorldRotation` (`self.Arrow`) (`KismetMathLibrary.Conv_VectorToRotator` (`self.MoveDirection`)) false false))

(fn `UserConstructionScript`)