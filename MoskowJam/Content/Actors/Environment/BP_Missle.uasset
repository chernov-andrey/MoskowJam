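; BP_Missle is a homing projectile (called a torpedo in its debug text) that notifies a Barrier when it hits one.
; On BeginPlay it homes on the Target's root component through ProjectileMovement, with a longer self-destruct timer than when no valid target exists.
; Sphere overlap or mesh hit with a Barrier calls MissileHitMessage and destroys the missile.
; SetTarget only stores the target, and Tick prints target and position for debugging.
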(event `self.ReceiveBeginPlay`
  (`/Engine/EditorBlueprintResources/StandardMacros.IsValid` (`Actor.RootComponent` (`self.Target`))
    (:`Is Valid`
      (set `ProjectileMovementComponent.HomingTargetComponent` (`Actor.RootComponent` (`self.Target`)) (`self.ProjectileMovement`))
      (`KismetSystemLibrary.Delay` 30.0)
      (`self.K2_DestroyActor`))
    (:`Is Not Valid`
      (`KismetSystemLibrary.Delay` 15.0)
      (`self.K2_DestroyActor`))))

(event `self.ReceiveTick`
  (params (DeltaSeconds :type "Float (single-precision)"))
  (bind (_returnvalue_x _returnvalue_y _returnvalue_z) (`KismetMathLibrary.BreakVector` (`self.K2_GetActorLocation`)))
  (`KismetSystemLibrary.PrintString` (`KismetStringLibrary.Concat_StrStr` "Я торпеда, моя цель: " (`KismetSystemLibrary.GetDisplayName` (`self.Target`)) ", мои координаты: " (`KismetStringLibrary.Conv_DoubleToString` _returnvalue_x) "     " (`KismetStringLibrary.Conv_DoubleToString` _returnvalue_y) "     " (`KismetStringLibrary.Conv_DoubleToString` _returnvalue_z)) true true (struct :`G` 0.66 :`B` 1.0 :`A` 1.0) 0.0))

(event `self.Sphere.OnComponentBeginOverlap`
  (params (OverlappedComponent :type "PrimitiveComponent Object Reference") (OtherActor :type "Actor Object Reference") (OtherComp :type "PrimitiveComponent Object Reference") (OtherBodyIndex :type Integer) (bFromSweep :type Boolean) (SweepResult :type "HitResult Structure (by ref)"))
  (if (== (`GameplayStatics.GetObjectClass` OtherActor) "/Script/MoskowJam.Barrier")
    (message `/Game/Actors/Environment/Barrier/Traps/Traps_Iteractive/BI_InteractWithEnvironment.MissileHit` OtherActor)
    (`self.K2_DestroyActor`)))

(event `self.Missle.OnComponentHit`
  (params (HitComponent :type "PrimitiveComponent Object Reference") (OtherActor :type "Actor Object Reference") (OtherComp :type "PrimitiveComponent Object Reference") (NormalImpulse :type "Vector Structure") (Hit :type "HitResult Structure (by ref)"))
  (cast `Barrier` OtherActor)
  (message `/Game/Actors/Environment/Barrier/Traps/Traps_Iteractive/BI_InteractWithEnvironment.MissileHit` OtherActor)
  (`self.K2_DestroyActor`))

(event `/Game/Interfaces/IBP_Torpeda.Set Target`
  (params (Target :type "Barrier Object Reference"))
  (set `self.Target` Target))

(fn `UserConstructionScript`)