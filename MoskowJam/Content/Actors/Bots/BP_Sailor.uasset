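; Cat crew bot that works and rests at stations while tracking stamina and stress.
; Stamina and stress components update its cat card widget, seeded with NPC manager name and photo; max stress increments the game mode's angry-cat counter.
; Go/Anim gameplay tags hold task and animation state; relax transitions, including on exhaustion, write a random rest station to the AI blackboard.
; SetWorkTask is a stub, and Tick prints debug state.
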(event `self.ReceiveBeginPlay`
  ;[1 1 1] Со старта релаксируем
  (`self.Add Tag` (struct :`TagName` "Anim.Relax"))
  (bind _outactors (`GameplayStatics.GetAllActorsOfClass` "/Game/Actors/Environment/BP_NPC_Manager.BP_NPC_Manager_C"))
  (for _array_element _outactors
    (set `self.NPC Manager` _array_element))
  (bind _outitem (`/Game/Actors/Environment/BP_NPC_Manager.Get Cat Name` (`self.NPC Manager`)))
  (set `self.My Name` _outitem)
  (bind _outitem_2 (`/Game/Actors/Environment/BP_NPC_Manager.Get Cat Image` (`self.NPC Manager`)))
  (bind _output_get (set `self.My Photo` _outitem_2))
  (bind _returnvalue (`|CreateWidget` "/Game/GUI/BPW_Cat_Case.BPW_Cat_Case_C" null (`self.My Name`) _output_get))
  (`Widget.SetVisibility` _returnvalue "Hidden")
  (bind _output_get_2 (set `self.Cat Case` _returnvalue))
  (`UserWidget.AddToViewport` _output_get_2 0)
  ;[1 1 1] Поменялось значение стамины или стресса - обновляем виджеты
  (add `/Game/Components/CBP_Scale.Update Widget` (`self.Scale_Stamina`) (delegate `Update Stamina Widget`))
  (add `/Game/Components/CBP_Scale.Update Widget` (`self.Scale_Stress`) (delegate `Update Stress Widget`))
  ;[1 1 1] Меняем на 1 значения стамины и стресса, чтобы обновить виджеты
  (message `/Game/Interfaces/IBP_Scale_Interaction.Change` (`self.Scale_Stamina`) true 1.0)
  (message `/Game/Interfaces/IBP_Scale_Interaction.Change` (`self.Scale_Stress`) false 100.0)
  ;[1 1 1] Подписываемся на достижении стамины нуля и на достижении стресса максимума
  (add `/Game/Components/CBP_Scale.It is zero` (`self.Scale_Stamina`) (delegate `Stamina is Zero Helper`))
  (add `/Game/Components/CBP_Scale.it is max` (`self.Scale_Stress`) (delegate `Stress is Max Helper`)))

(event `Stress is Max Helper`
  ;[1 1 1] Подписываемся на достижении стамины нуля и на достижении стресса максимума
  ;;[1 1 1] Вызываем функцию гейммода, если у нас появился кот с максимальным стрессом
  (bind _asbp_game_mode_base_mj (`/Game/Library/FL_General.Get MJ GameMode`))
  (`/Game/GameSettings/BP_GameModeBase_MJ.Increase Angry Cats Counter` _asbp_game_mode_base_mj))

(event `/Game/Interfaces/IBP_HR.Increase Stress`
  (params (`Increase Stress` :type "Float (double-precision)"))
  (message `/Game/Interfaces/IBP_Scale_Interaction.Change` (`self.Scale_Stress`) true `Increase Stress`))

(event `Update Stamina Widget`
  (params (Percent :type "Float (double-precision)"))
  ;[1 1 1] Поменялось значение стамины или стресса - обновляем виджеты
  (`/Game/GUI/BPW_Cat_Case.Set Percent Stamina` (`self.Cat Case`) Percent))

(event `Update Stress Widget`
  (params (Percent :type "Float (double-precision)"))
  ;[1 1 1] Поменялось значение стамины или стресса - обновляем виджеты
  (`/Game/GUI/BPW_Cat_Case.Set Percent Stress` (`self.Cat Case`) Percent))

(event `Stamina is Zero Helper`
  ;[1 1 1] Подписываемся на достижении стамины нуля и на достижении стресса максимума
  (bind _removed (`self.Remove Tag` (`self.Work Tag`)))
  (if _removed
    (`self.Add Tag` (struct :`TagName` "Go.ToRelax.Place1"))))

(event `/Game/Interfaces/IBP_HR.Regen Stamina`
  (params (`Regen Value` :type "Float (double-precision)"))
  (message `/Game/Interfaces/IBP_Scale_Interaction.Change` (`self.Scale_Stamina`) true `Regen Value`))

(event `/Game/Interfaces/IBP_HR.Regen Stress`
  (params (`Regen Value` :type "Float (double-precision)"))
  (message `/Game/Interfaces/IBP_Scale_Interaction.Change` (`self.Scale_Stress`) false `Regen Value`))

(event `/Game/Interfaces/IBP_HR.Work Result Message`
  (params (Message :type Text))
  (bind _cat_message_widget (`/Game/Library/FL_General.Create Cat Message` (`self.My Name`) (`self.My Photo`) Message))
  (add `/Game/GUI/BPW_Cat_Message.Destroy This Actor` _cat_message_widget (delegate `Destory this actor helper`)))

(event `Destory this actor helper`
  (`Widget.RemoveFromParent` (stale `/Game/Interfaces/IBP_HR.Work Result Message` _cat_message_widget)))

(event `self.ReceiveTick`
  (params (DeltaSeconds :type "Float (single-precision)"))
  (`KismetSystemLibrary.PrintString` (`KismetStringLibrary.Concat_StrStr` "Я кот: " (`KismetSystemLibrary.GetDisplayName` self) ", я иду " (`KismetStringLibrary.Conv_NameToString` (`BlueprintGameplayTagLibrary.GetTagName` (`self.Work Tag`))) ", сейчас я " (`KismetStringLibrary.Conv_NameToString` (`BlueprintGameplayTagLibrary.GetTagName` (`self.Anim Tag`)))) true true (struct :`G` 0.66 :`B` 1.0 :`A` 1.0) 0.0))

(fn `Add Tag`
  (params (`Add Tag` :type "GameplayTag Structure"))
  (returns (Added :type Boolean))
  (locals (`New Tag` :type "GameplayTag Structure"))
  (bind _output_get (set `local.New Tag` `Add Tag`))
  (if (`BlueprintGameplayTagLibrary.MatchesTag` _output_get (struct :`TagName` "Go"))
    (set `self.Work Tag` (`local.New Tag`)))
  (if (`BlueprintGameplayTagLibrary.MatchesTag` _output_get (struct :`TagName` "Anim"))
    (set `self.Anim Tag` (`local.New Tag`)))
  (`BlueprintGameplayTagLibrary.AddGameplayTag` (`self.TagContainer`) (`local.New Tag`))
  (`KismetSystemLibrary.PrintString` (`KismetStringLibrary.Conv_NameToString` (`BlueprintGameplayTagLibrary.GetTagName` (`local.New Tag`))) true true (struct :`R` 1.0 :`B` 0.136101 :`A` 1.0) 10.0)
  (`|SwitchGameplayTag` (`local.New Tag`)
    (:`Default`
      _)
    (:`Go.ToRelax`
      (`self.Clear PlaceToWork`)
      (`self.Set PlaceToRelax`)))
  (return true))

(fn `Clear PlaceToWork`
  (locals (`Clear Object` :type "Object Object Reference"))
  (`BlackboardComponent.SetValueAsObject` (`AIBlueprintHelperLibrary.GetBlackboard` (`self.GetController`)) (`self.PlaceToWork`) (`local.Clear Object`)))

(fn `Damage Stamina`
  (params (`Damage Stamina` :type "Float (double-precision)"))
  (returns (`Not Enought` :type Boolean))
  (bind _enought (`/Game/Components/CBP_Scale.Enought to Decrease?` (`self.Scale_Stamina`) `Damage Stamina`))
  (if _enought
    (message `/Game/Interfaces/IBP_Scale_Interaction.Change` (`self.Scale_Stamina`) false `Damage Stamina`))
  (return _enought))

(fn `Damage Stamina_1_1`)

(fn `Get Anim Tag`
  (returns (`Anim Tag` :type "GameplayTag Structure"))
  (return (`self.Anim Tag`)))

(fn `Get Scale Stamina Component`
  (returns (Scale_Stamina :type "/Game/Components/CBP_Scale Object Reference"))
  (return (`self.Scale_Stamina`)))

(fn `Get Scale Stress Component`
  (returns (Scale_Stress :type "/Game/Components/CBP_Scale Object Reference"))
  (return (`self.Scale_Stress`)))

(fn `Get Work Tag`
  (returns (`Work Tag` :type "GameplayTag Structure"))
  (return (`self.Work Tag`)))

(fn `Has Tag`
  (params (`Has Tag` :type "GameplayTag Structure") (`Exect Match` :type Boolean))
  (returns (Has :type Boolean))
  (return (`BlueprintGameplayTagLibrary.HasTag` (`self.TagContainer`) `Has Tag` `Exect Match`)))

(fn `Read Case`
  (returns (`Cat Case` :type "/Game/GUI/BPW_Cat_Case Object Reference"))
  (return (`self.Cat Case`)))

(fn `Remove Tag`
  (params (`Remove Tag` :type "GameplayTag Structure"))
  (returns (Removed :type Boolean))
  (locals (`Removed Tag` :type "GameplayTag Structure"))
  (bind _output_get (set `local.Removed Tag` `Remove Tag`))
  (bind _returnvalue (`BlueprintGameplayTagLibrary.RemoveGameplayTag` (`self.TagContainer`) _output_get))
  (if _returnvalue
    (if (`BlueprintGameplayTagLibrary.MatchesTag` (`local.Removed Tag`) (struct :`TagName` "Go"))
      (set `self.Work Tag` (struct))
      (return true)
      (else
        (if (`BlueprintGameplayTagLibrary.MatchesTag` (`local.Removed Tag`) (struct :`TagName` "Anim"))
          (set `self.Anim Tag` (struct)))
        (if (`BlueprintGameplayTagLibrary.MatchesTag` (`local.Removed Tag`) (struct :`TagName` "Anim.Working"))
          (`self.Clear PlaceToWork`)
          (`self.Set PlaceToRelax`)
          (return false)
          (else
            (return true)))))))

(fn `Set PlaceToRelax`
  (locals (PlaceToRelax :type Name :default "PlaceToRelax") (`Place 1` :type "GameplayTag Structure" :default (struct :`TagName` "Go.ToRelax.Place1")) (`Place 2` :type "GameplayTag Structure" :default (struct :`TagName` "Go.ToRelax.Place2")) (`Place 3` :type "GameplayTag Structure" :default (struct :`TagName` "Go.ToRelax.Place3")) (`Place Tag` :type Name :default "Relax #1"))
  (bind _returnvalue (select `int` (`KismetMathLibrary.RandomIntegerInRange` 0 2) :`0` (`local.Place 1`) :`1` (`local.Place 2`) :`2` (`local.Place 3`)))
  (`self.Add Tag` _returnvalue)
  (`|SwitchGameplayTag` _returnvalue
    (:`Go.ToRelax.Place1`
      (set `local.Place Tag` "Relax #1"))
    (:`Go.ToRelax.Place2`
      (set `local.Place Tag` "Relax #2"))
    (:`Go.ToRelax.Place3`
      (set `local.Place Tag` "Relax #3")))
  (bind _outactors (`GameplayStatics.GetAllActorsOfClassWithTag` "/Game/Actors/Environment/BP_WorkPlace.BP_WorkPlace_C" (`local.Place Tag`)))
  (bind _output (`|GetArrayItem` _outactors))
  (`BlackboardComponent.SetValueAsObject` (`AIBlueprintHelperLibrary.GetBlackboard` (`self.GetController`)) (`local.PlaceToRelax`) _output)
  (`/Game/Interfaces/IBP_HR.Activate WorkStation` _output))

(fn `Set PlaceToWork`
  (params (ObjectValue :type "Object Object Reference"))
  (`BlackboardComponent.SetValueAsObject` (`AIBlueprintHelperLibrary.GetBlackboard` (`self.GetController`)) (`self.PlaceToWork`) ObjectValue))

(fn `Set Work Task`
  (params (ThisPlace :type "Object Object Reference") (ThisWorkReqTag :type "GameplayTag Structure") (`Stamina Cost` :type "Float (double-precision)") (`Stress Cost` :type "Float (double-precision)"))
  (returns (`Work set` :type Boolean))
  (return false))

(fn `UserConstructionScript`)