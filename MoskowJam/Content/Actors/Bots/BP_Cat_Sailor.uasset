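; Cat sailor bot actor that can visibly carry torpedoes, built on a parent Blueprint that supplies the base setup.
; On BeginPlay it runs the parent logic, clears its torpedo flag and gives the mesh a random material from the CatColor array for coat variety.
; It binds to the ChangeTorpedoVisibility dispatcher, which shows or hides its static mesh, likely the carried torpedo.
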(event `self.ReceiveBeginPlay`
  (`parent.ReceiveBeginPlay`)
  (`self. Set Have Torpedos` false)
  (`PrimitiveComponent.SetMaterial` (`self.Mesh`) 0 (`KismetArrayLibrary.Array_Random` (`self.Cat Color`)))
  (add `self.Change Torpedo Visibility` (delegate `Change Torpedo Visibility_событие`)))

(event `Change Torpedo Visibility_событие` :!signature `self.Change Torpedo Visibility`
  (params (Visible :type Boolean))
  (`SceneComponent.SetVisibility` (`self.StaticMesh`) Visible false))

(fn `UserConstructionScript`
  (`parent.UserConstructionScript`))