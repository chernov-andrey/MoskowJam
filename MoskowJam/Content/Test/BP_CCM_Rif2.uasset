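; BP_CCM_Rif2 is a Chaos cache manager Blueprint that triggers cached playback for the Rif component, then removes itself.
; BeginPlay assigns the CCC_Rif_2 cache collection, and the construction script leaves the root Movable.
; TriggerRIF makes the root Static, reapplies the actor's current location to it and Rif, and calls TriggerAll.
; The actor destroys itself after a short delay.
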(event `self.ReceiveBeginPlay`
  (`self.SetCacheCollection` self "/Game/Test/CCC_Rif_2.CCC_Rif_2"))

(event `/Game/Interfaces/IBP_Test_Rif.Trigger RIF`
  (set `self.Location Buffer` (`self.K2_GetActorLocation` self))
  (`SceneComponent.SetMobility` (`self.RootComponent`) "Static")
  (`self.K2_SetActorLocation` self (`self.Location Buffer`) false false)
  (`SceneComponent.K2_SetWorldLocation` (`self.Rif`) (`self.Location Buffer`) false false)
  (`self.TriggerAll`)
  (`KismetSystemLibrary.Delay` 5.0)
  (`self.K2_DestroyActor`))

(fn `UserConstructionScript`
  (`SceneComponent.SetMobility` (`self.RootComponent`) "Movable"))