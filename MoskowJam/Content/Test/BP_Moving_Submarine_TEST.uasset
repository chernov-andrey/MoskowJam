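; Test submarine pawn that drives forward, turns in short timed bursts, tracks a torpedo count and handles hull breaches.
; Engine speed feeds Tick movement input, RotatingMovement performs turns, and torpedo load and launch events only adjust the counter and print.
; Damage raises the attached BP_Water hole count and spawns a BP_PlayerWorkPlace at a random free SinkBox.
; Healing a hole lowers that count, frees the box and destroys the station.
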(event `self.ReceiveBeginPlay`
  (bind _returnvalue (`|SpawnActorFromClass` "/Game/Actors/Environment/Volume/BP_Water.BP_Water_C" (`KismetMathLibrary.Conv_VectorToTransform` (`self.K2_GetActorLocation`)) "Undefined" "MultiplyWithRoot" self null))
  (bind _output_get (set `self.Water Volume` _returnvalue))
  (`self.K2_AttachToActor` _output_get self "None" "KeepRelative" "KeepRelative" "KeepRelative" false)
  (`BlueprintSetLibrary.Set_AddItems` (`self.Array of Water Sink`) (`|MakeArray` (`self.Sink Box 1`) (`self.Sink Box 2`) (`self.Sink Box 3`) (`self.Sink Box 4`) :!type "ActorComponent Object Reference")))

(event `self.ReceiveTick`
  (params (DeltaSeconds :type "Float (single-precision)"))
  ;[1 1 1] Двигаем подлодку вперед при нажатии на кнопку Z
  (if (`self.MoveForward`)
    (`self.AddMovementInput` (`self.GetActorForwardVector`) (`self.scale_speed`))))

(event `self.Turn`
  (params (Right :type Boolean))
  ;[1 1 1] Вращает подлодку с постоянным углом, пока мы не отменим (Отмена не настроена)
  (if Right
    (set `self.scale_turn` 10.0)
    (else
      (set `self.scale_turn` -10.0)))
  (set `RotatingMovementComponent.RotationRate` (`KismetMathLibrary.MakeRotator` 0.0 0.0 (`self.scale_turn`)) (`self.RotatingMovement`))
  (`KismetSystemLibrary.Delay` 0.2)
  (set `RotatingMovementComponent.RotationRate` (struct) (`self.RotatingMovement`)))

(event `self.Engine`
  (params (Speed :type "Float (double-precision)"))
  (set `self.scale_speed` Speed)
  (set `self.MoveForward` true))

(event `self.:aunch Torpedos`
  (`/Game/Components/CBP_Items_Integer.Dec Object` (`self.Torpedos`))
  (`KismetSystemLibrary.PrintString` "Торпеда запущена"))

(event `self.Load Torpedos`
  (`/Game/Components/CBP_Items_Integer.Inc Object` (`self.Torpedos`))
  (`KismetSystemLibrary.PrintString` "Торпеда заряжена"))

(event `self.Damage Taken`
  (`/Game/Actors/Environment/Volume/BP_Water.Change Nims of Holes` (`self.Water Volume`) true)
  (bind _output_get (set `self.Random` (`KismetMathLibrary.RandomInteger` 4) :!label _label))
  (switch `int` _output_get
    (:`0`
      (set `self.Sink Box Var` (`self.Sink Box 1`)))
    (:`1`
      (set `self.Sink Box Var` (`self.Sink Box 2`)))
    (:`2`
      (set `self.Sink Box Var` (`self.Sink Box 3`)))
    (:`3`
      (set `self.Sink Box Var` (`self.Sink Box 4`))))
  (if (`BlueprintSetLibrary.Set_Contains` (`self.Array of Water Sink`) (`self.Sink Box Var`))
    (bind _returnvalue (`BlueprintSetLibrary.Set_Remove` (`self.Array of Water Sink`) (`self.Sink Box Var`)))
    (if _returnvalue
      (bind _returnvalue_2 (`|SpawnActorFromClass` "/Game/Actors/Environment/Player_WorkPlace/BP_PlayerWorkPlace.BP_PlayerWorkPlace_C" (`KismetMathLibrary.Conv_VectorToTransform` (`SceneComponent.K2_GetComponentLocation` (`self.Sink Box Var`))) "Undefined" "MultiplyWithRoot" null "NewEnumerator8" null))
      (`BlueprintMapLibrary.Map_Add` (`self.Sink Place`) _returnvalue_2 (make `/Game/Structures/ST_Sink_Place` (`self.Sink Box Var`) true)))
    (elif (`BlueprintSetLibrary.Set_IsNotEmpty` (`self.Array of Water Sink`))
      (goto _label))))

(event `self.Hole Heal`
  (params (`This Hole` :type "/Game/Actors/Environment/Player_WorkPlace/BP_PlayerWorkPlace Object Reference"))
  (`/Game/Actors/Environment/Volume/BP_Water.Change Nims of Holes` (`self.Water Volume`) false)
  (`BlueprintSetLibrary.Set_Add` (`self.Array of Water Sink`) (break `/Game/Structures/ST_Sink_Place` (`BlueprintMapLibrary.Map_Find` (`self.Sink Place`) `This Hole`)))
  (`self.K2_DestroyActor` `This Hole`))

(event `self.Box.OnComponentHit`
  (params (HitComponent :type "PrimitiveComponent Object Reference") (OtherActor :type "Actor Object Reference") (OtherComp :type "PrimitiveComponent Object Reference") (NormalImpulse :type "Vector Structure") (Hit :type "HitResult Structure (by ref)"))
  (`KismetSystemLibrary.PrintString` (`KismetSystemLibrary.GetDisplayName` HitComponent) true true (struct :`G` 0.082607 :`B` 1.0 :`A` 1.0)))

(event `self.StaticMesh.OnComponentHit`
  (params (HitComponent :type "PrimitiveComponent Object Reference") (OtherActor :type "Actor Object Reference") (OtherComp :type "PrimitiveComponent Object Reference") (NormalImpulse :type "Vector Structure") (Hit :type "HitResult Structure (by ref)"))
  (`KismetSystemLibrary.PrintString` (`KismetSystemLibrary.GetDisplayName` HitComponent) true true (struct :`R` 1.0 :`G` 0.014728 :`A` 1.0)))

(event `self.Box1.OnComponentHit`
  (params (HitComponent :type "PrimitiveComponent Object Reference") (OtherActor :type "Actor Object Reference") (OtherComp :type "PrimitiveComponent Object Reference") (NormalImpulse :type "Vector Structure") (Hit :type "HitResult Structure (by ref)"))
  (`KismetSystemLibrary.PrintString` (`KismetSystemLibrary.GetDisplayName` HitComponent) true true (struct :`G` 1.0 :`B` 0.159457 :`A` 1.0)))

(fn `Dec Torpedos Prepared`
  (`/Engine/EditorBlueprintResources/StandardMacros.DecrementInt` (`self.Torpedos Prepared`)))

(fn `Decrease Water Level`
  (`/Game/Actors/Environment/Volume/BP_Water.Decrease Water Level` (`self.Water Volume`)))

(fn `Get PawnMovement`
  (returns (FloatingPawnMovement :type "FloatingPawnMovement Object Reference"))
  (return (`self.FloatingPawnMovement`)))

(fn `Get Random Point in Volume of Component`
  (params (`Цель` :type "BoxComponent Object Reference"))
  (returns (ReturnValue :type "Vector Structure"))
  (bind (_returnvalue_x _returnvalue_y _returnvalue_z) (`KismetMathLibrary.BreakVector` (`SceneComponent.K2_GetComponentLocation` `Цель`)))
  (bind (_returnvalue_x_2 _returnvalue_y_2 _returnvalue_z_2) (`KismetMathLibrary.BreakVector` (`BoxComponent.GetScaledBoxExtent` `Цель`)))
  (return (`KismetMathLibrary.MakeVector` (`KismetMathLibrary.RandomFloatInRange` (- _returnvalue_x _returnvalue_x_2) _returnvalue_x_2) (`KismetMathLibrary.RandomFloatInRange` (- _returnvalue_y _returnvalue_y_2) _returnvalue_y_2) (`KismetMathLibrary.RandomFloatInRange` (- _returnvalue_z _returnvalue_z_2) _returnvalue_z_2))))

(fn `Inc Torpedos Prepared`
  (`/Engine/EditorBlueprintResources/StandardMacros.IncrementInt` (`self.Torpedos Prepared`)))

(fn `Max Torpedos?`
  (returns (`Max Torpedos` :type Boolean))
  (bind _more_than_max (`/Game/Components/CBP_Items_Integer.More than max?` (`self.Torpedos`)))
  (return _more_than_max))

(fn `Move This Sub`
  (params (MoveForward :type Boolean))
  (set `self.MoveForward` MoveForward))

(fn `Torpedos More than Max`
  (returns (`More than Max` :type Boolean))
  (return (>= (`self.Torpedos Prepared`) (`self.Max Torpedos Prepared`))))

(fn `Torpedos Zero`
  (returns (ReturnValue :type Boolean))
  (return (<= (`self.Torpedos Prepared`) 0)))

(fn `UserConstructionScript`
  (`/Game/Components/CBP_Items_Integer.Set Object Max` (`self.Torpedos`) 5)
  (`/Game/Components/CBP_Items_Integer.Set Object` (`self.Torpedos`) 0))

(fn `Zero Torpedos?`
  (returns (`Zero Torpedos` :type Boolean))
  (bind _returnvalue (`/Game/Components/CBP_Items_Integer.Zero?` (`self.Torpedos`)))
  (return _returnvalue))