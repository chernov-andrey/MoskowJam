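; Radar actor that shows a single tracked target, such as a spawned trap, on a dynamic display material with a looping rotation.
; BeginPlay binds to every Spawner's spawn-trap event, which replaces the current target.
; Show_target picks a stone icon for destructible objects and reefs, or a shark icon for sharks.
; Tick shows the blip within a square Distance range, feeding normalized X/Y offsets, swapped, into material parameters.
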(event `self.ReceiveBeginPlay`
  (`|ExecutionSequence`
    (:`then_0`
      (bind _returnvalue (`KismetMaterialLibrary.CreateDynamicMaterialInstance` "/Game/Test/M_RadarDisplay.M_RadarDisplay" "None"))
      (bind _output_get (set `self.M_Instance` _returnvalue))
      (`PrimitiveComponent.SetMaterial` (`self.Cube`) 1 _output_get)
      (`MaterialInstanceDynamic.SetTextureParameterValue` _output_get "Param" "/Game/ART/Images/Button.Button")
      (bind (_direction _newtrack_0) (`Timeline|Timeline` :!via `PlayFromStart` :!label _label)
        (:`Update`
          (`MaterialInstanceDynamic.SetScalarParameterValue` _output_get "Rotation" _newtrack_0))
        (:`Finished`
          (if true
            (goto _label :!via `PlayFromStart`)))))
    (:`then_1`
      (bind _outactors (`GameplayStatics.GetAllActorsOfClass` "/Script/MoskowJam.Spawner"))
      (for _array_element _outactors
        (add `Spawner.OnSpawnTrapEvent` _array_element (delegate `SpawnTrap`))))))

(event `SpawnTrap`
  (params (CounterTrap :type Integer) (Traps :type "Barrier Object Reference"))
  (bind _output_get (set `self.Target` Traps))
  (`self.Show_target` _output_get))

(event `self.ReceiveTick`
  (params (DeltaSeconds :type "Float (single-precision)"))
  (bind (_returnvalue_x _returnvalue_y) (`KismetMathLibrary.BreakVector` (`self.K2_GetActorLocation`)))
  (bind _distance (`self.Distance`))
  (bind _m_instance (`self.M_Instance`))
  (bind _target (`self.Target`))
  (bind (_returnvalue_x_2 _returnvalue_y_2) (`KismetMathLibrary.BreakVector` (`self.K2_GetActorLocation` _target)))
  (bind _returnvalue (- _returnvalue_y_2 _returnvalue_y))
  (bind _returnvalue_2 (- _returnvalue_x_2 _returnvalue_x))
  (`/Engine/EditorBlueprintResources/StandardMacros.IsValid` _target
    (:`Is Valid`
      (if (and (<= (`KismetMathLibrary.Abs` _returnvalue_2) _distance) (<= (`KismetMathLibrary.Abs` _returnvalue) _distance))
        (`MaterialInstanceDynamic.SetScalarParameterValue` _m_instance "ShowTarget" 1.0)
        (`MaterialInstanceDynamic.SetScalarParameterValue` (`self.M_Instance`) "Y_Target" (/ _returnvalue_2 _distance))
        (`MaterialInstanceDynamic.SetScalarParameterValue` (`self.M_Instance`) "X_Target" (/ _returnvalue _distance))
        (else
          (`MaterialInstanceDynamic.SetScalarParameterValue` _m_instance "ShowTarget" 0.0))))
    (:`Is Not Valid`
      (`MaterialInstanceDynamic.SetScalarParameterValue` (`self.M_Instance`) "ShowTarget" 0.0))))

(event `Show_target`
  (params (BarrierDetected :type "Barrier Object Reference"))
  (bind _output_get (set `self.Target` BarrierDetected))
  (cast `/Game/Actors/Environment/Barrier/Traps/Traps_Iteractive/BP_DestructibleObject` _output_get
    (:`then`
      (`MaterialInstanceDynamic.SetTextureParameterValue` (`self.M_Instance`) "Param" "/Game/Test/Stone2.Stone2"))
    (:`CastFailed`
      (cast `/Game/Actors/Environment/Barrier/Traps/BP_Rifs` _output_get
        (:`then`
          (`MaterialInstanceDynamic.SetTextureParameterValue` (`self.M_Instance`) "Param" "/Game/Test/Stone2.Stone2"))
        (:`CastFailed`
          (cast `/Game/Actors/Environment/Barrier/Traps/Traps_Iteractive/Creatures/BP_Creature_Shark` _output_get)
          (`MaterialInstanceDynamic.SetTextureParameterValue` (`self.M_Instance`) "Param" "/Game/Test/Shark.Shark"))))))

(fn `UserConstructionScript`)