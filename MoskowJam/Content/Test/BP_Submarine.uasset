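; Submarine actor that detects reef obstacles (BP_Rifs) and launches missiles.
; Three seconds after BeginPlay it triggers a team mood change, disarms the missile, and caches the Sphere and BarierDetector world locations once.
; BarierDetector overlaps with reefs broadcast located and end-of-location events.
; Exposed functions get or set the armed flag, return the cached detector location, and spawn BP_Missle at the cached point, then disarm without checking the flag.
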(event `self.ReceiveBeginPlay`
  (`KismetSystemLibrary.Delay` 3.0)
  (`self.Change_MoodOfTheTeam`)
  (set `self.Missle Armed` false)
  (set `self.Missle Spawn Location` (`SceneComponent.K2_GetComponentLocation` (`self.Sphere`)))
  (set `self.Barier Detector Location` (`SceneComponent.K2_GetComponentLocation` (`self.Barier Detector`))))

(event `self.Barier Detector.OnComponentBeginOverlap`
  (params (OverlappedComponent :type "PrimitiveComponent Object Reference") (OtherActor :type "Actor Object Reference") (OtherComp :type "PrimitiveComponent Object Reference") (OtherBodyIndex :type Integer) (bFromSweep :type Boolean) (SweepResult :type "HitResult Structure (by ref)"))
  (cast `/Game/Actors/Environment/Barrier/Traps/BP_Rifs` OtherActor)
  (`self.Barier Located`))

(event `self.Barier Detector.OnComponentEndOverlap`
  (params (OverlappedComponent :type "PrimitiveComponent Object Reference") (OtherActor :type "Actor Object Reference") (OtherComp :type "PrimitiveComponent Object Reference") (OtherBodyIndex :type Integer))
  (cast `/Game/Actors/Environment/Barrier/Traps/BP_Rifs` OtherActor)
  (`self.End of Location`))

(fn `Get Barier Location`
  (returns (`Barier Detector Location` :type "Vector Structure"))
  (return (`self.Barier Detector Location`)))

(fn `Get is Missle Armed`
  (returns (`Missle Armed` :type Boolean))
  (return (`self.Missle Armed`)))

(fn `Set is Missle Armed`
  (params (`Missle Armed` :type Boolean))
  (set `self.Missle Armed` `Missle Armed`))

(fn `Spawn Missle`
  (`|SpawnActorFromClass` "/Game/Actors/Environment/BP_Missle.BP_Missle_C" (`KismetMathLibrary.MakeTransform` (`self.Missle Spawn Location`)) "Undefined" "MultiplyWithRoot" self null)
  (`self.Set is Missle Armed` false))

(fn `UserConstructionScript`)